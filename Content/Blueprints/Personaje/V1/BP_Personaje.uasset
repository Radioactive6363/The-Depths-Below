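; First-person player character that moves, looks, climbs ladders, pauses and repairs broken glass, engine and oxygen tank parts.
; Tick switches idle/walk camera shakes by velocity; timelines step ladder climbs with input disabled.
; Short camera traces drive interaction, with consoles locking movement and look.
; Click repairs pass tagged component names to target actors, gated by extraction state or held tool; engine welding also checks click hold time.
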(event Custom|CameraShakeEvent
  ;[1 1 1] Camera Shake
  (if (|CondicionVelocidad)
    (|DetenerShakeCamaraCorriendo)
    (|ComenzarShakeCamaraIdle)
    (elif (not (Variables|Default|GetEscalera))
      (|ComenzarShakeCamaraCorriendo))))

(event EventTick
  (params (DeltaSeconds :type Float%20%28single-precision%29))
  ;[1 1 1] Camera Shake
  (CallFunction|CameraShakeEvent)
  (|MousealMediodelaPantallaalPausar))

(event Input|ActionEvents|InputActionInteractuar
  (params (Key :type Key%20Structure :default "None"))
  ;[1 1 1] Interaccion con Objetos
  (:Pressed
    (bind (_returnvalue _outhit) (|LineaInteraccion))
    (if _returnvalue
      (if (.ReturnValue (|ActorInteractuado _outhit))
        (|ActoresConsola)
        (else
          (|ActoresObjeto (.ReturnValue2 (|ActorInteractuado _outhit)))))
      (Class|BPInterfaces|Interact(Message) (.HitActor (|ActorInteractuado _outhit))))))

(event Input|ActionEvents|InputActionPausa
  (params (Key :type Key%20Structure :default "None"))
  ;[1 1 1] Menu Pausa
  (:Pressed
    (if (Variables|Default|GetVivo)
      (|ChequeoPausaCreada
        (:Is%20Valid
          _)
        (:Is%20Not%20Valid
          (bind _returnvalue (UserInterface|CreateWidget "/Game/Blueprints/UI/Menu/BP_PauseMenu.BP_PauseMenu_C"))
          (Variables|Default|SetPausado _returnvalue)))
      (if (Game|IsGamePaused)
        (|Despausar)
        (if (Variables|Default|GetMouse)
          (goto _label execute2)
          (else
            (|RespetarEstadoPreviodeInput :!label _label)))
        (else
          (|Pausar (Variables|/Game/Blueprints/UI/Menu/BP_PauseMenu.BP_PauseMenu_C|GetHorizontalBox_69 _returnvalue) (Variables|/Game/Blueprints/UI/Menu/BP_PauseMenu.BP_PauseMenu_C|GetVerticalBox_157 _returnvalue)))))))

(event Input|ActionEvents|InputActionClick
  (params (Key :type Key%20Structure :default "None"))
  ;[1 1 1] Interaccion Arreglos
  (:Pressed
    (if (Variables|Default|Getextraccion)
      (bind _returnvalue (Actor|GetActorOfClass "/Game/Blueprints/Objetos/V1/BP_Vidrio.BP_Vidrio_C"))
      (bind (_returnvalue_2 _outhit) (|LineaArregloVidrio))
      (if _returnvalue_2
        (if (.ReturnValue (|ParteseadelVidrio _outhit))
          (|ParteparaArreglar (.ReturnValue2 (|ParteseadelVidrio _outhit)))
          (Class|BPInterfaces|Interact(Message) _returnvalue)))
      (else
        (bind _returnvalue_3 (|ArregloMotor)
          (:then
            (bind (_returnvalue_4 _outhit_2) (|LineaArregloMotor :!label _label))
            (if _returnvalue_4
              (Audio|PlaySound2D "/Game/Audio/Welding.Welding" 1.0 1.0 0.0 0 0)
              (if (.ReturnValue (|ParteRotaseadelMotor _outhit_2))
                (if (Variables|Default|Getarreglando)
                  (Variables|Default|Setarreglando false)
                  (|ParteaArreglar (.ReturnValue2 (|ParteRotaseadelMotor _outhit_2)))
                  (Class|BPInterfaces|Interact(Message) _returnvalue_3)
                  (else
                    (|ChequeoTiempoMantenerClick Key)
                    (Variables|Default|Setarreglando true)
                    (goto _label))))
              (else
                (Variables|Default|Setarreglando false))))
          (:else
            (bind _returnvalue_5 (|ArregloTanque))
            (bind (_returnvalue_6 _outhit_3) (|LineaArregloTanque))
            (if _returnvalue_6
              (if (.ReturnValue (|ParteseadelTanque _outhit_3))
                (|PartequeArreglar (.ReturnValue2 (|ParteseadelTanque _outhit_3)))
                (Class|BPInterfaces|Interact(Message) _returnvalue_5)))))))))

(event Input|AxisEvents|InputAxisgirar
  (params (AxisValue :type Float%20%28single-precision%29))
  ;[1 1 1] Camara
  (|ChequeoEstadoInteraccion
    (:else
      (|MovimientoCamara AxisValue (stale Input|AxisEvents|InputAxismirararriba AxisValue)))))

(event Input|AxisEvents|InputAxismirararriba
  (params (AxisValue :type Float%20%28single-precision%29))
  ;[1 1 1] Camara
)

(event Input|AxisEvents|InputAxisderecha
  (params (AxisValue :type Float%20%28single-precision%29))
  (bind (_returnvalue _returnvalue2) (|DireccionaMoverse))
  ;[1 1 1] Movimiento
  (|ChequeoEscalera
    (:then
      ;[1 1 1] En Escalera
      (if _returnvalue
        (if (|AlturaMaximaParaSubir)
          (|Subir))
        (elif _returnvalue2
          (if (|AlturaMinimaParaBajar)
            (|Bajar)))))
    (:else
      (|MovimientoJugador AxisValue (stale Input|AxisEvents|InputAxisadelante AxisValue)))))

(event Input|AxisEvents|InputAxisadelante
  (params (AxisValue :type Float%20%28single-precision%29))
  ;[1 1 1] Movimiento
)

(fn ConstructionScript)