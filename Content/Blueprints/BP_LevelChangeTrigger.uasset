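; Level exit trigger: one volume plays an approaching-station sound for the player, another ends the level.
; The exit, also callable via ForceChangeLevel, fades the camera out, starts a timer and saves collectible and resource-terminal widget data to BP_Instance.
; The next level number, parsed from the map name, is stored for continuing.
; After the timer, it opens CheckPoint, or shows a paused victory screen after the final level.
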(event OnComponentBeginOverlap(TriggerSound)
  (params (OverlappedComponent :type Primitive%20Component%20Object%20Reference) (OtherActor :type Actor%20Object%20Reference) (OtherComp :type Primitive%20Component%20Object%20Reference) (OtherBodyIndex :type Integer) (bFromSweep :type Boolean) (SweepResult :type Hit%20Result%20Structure%20%28by%20ref%29))
  (if (== OtherActor (Game|GetPlayerCharacter 0))
    (Audio|PlaySound2D "/Game/Audio/AproximandoseEstacion.AproximandoseEstacion" 1.0 1.0 0.0 0 0)))

(event OnComponentBeginOverlap(TriggerChangeLevel)
  (params (OverlappedComponent :type Primitive%20Component%20Object%20Reference) (OtherActor :type Actor%20Object%20Reference) (OtherComp :type Primitive%20Component%20Object%20Reference) (OtherBodyIndex :type Integer) (bFromSweep :type Boolean) (SweepResult :type Hit%20Result%20Structure%20%28by%20ref%29))
  (bind _tiempodecambiodenivel (Variables|Default|GetTiempoDeCambioDeNivel))
  (if (== OtherActor (Game|GetPlayerCharacter 0))
    (CameraFades|StartCameraFade :self (Game|GetPlayerCameraManager 0) :ToAlpha 1.0 :Duration _tiempodecambiodenivel :bHoldWhenFinished true)
    (Utilities|Time|SetTimerbyEvent (delegate Custom|Cambio%20de%20Nivel) _tiempodecambiodenivel)
    (|EnviarDatosaInstancia)))

(event Custom|Cambio%20de%20Nivel
  (bind _returnvalue (Game|GetCurrentLevelName true))
  (if (< (+ (Math|Conversions|ToInteger(Byte) (Utilities|String|GetSubstring _returnvalue 5)) 1) 5)
    (Game|OpenLevel(byName) "CheckPoint")
    (else
      (|PantallaVictoria))))

(event Custom|ForceChangeLevel
  (bind _tiempodecambiodenivel (Variables|Default|GetTiempoDeCambioDeNivel))
  (CameraFades|StartCameraFade :self (Game|GetPlayerCameraManager 0) :ToAlpha 1.0 :Duration _tiempodecambiodenivel :bHoldWhenFinished true)
  (Utilities|Time|SetTimerbyEvent (delegate Custom|Cambio%20de%20Nivel) _tiempodecambiodenivel)
  (|EnviarDatosaInstancia))

(fn ConstructionScript)