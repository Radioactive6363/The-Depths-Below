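; Game mode for an underwater horror game, running ambient sound, random scares, attacks and defeat.
; Outside the tutorial, Level4 and checkpoint maps, a looping timer picks flickering lights, with or without monster roars, or random audio.
; EventoAtaque stages an attack with water flow, motor or oxygen breakage, impact, alarm and monster sounds, then restores lights.
; Derrota copies current depth from the monitor UI into the game instance and opens the Lose level.
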(event Custom|EventosAleatorios%20-%20Selector
  (bind _lightsflickeringtimermax (Variables|Default|GetLightsFlickeringTimerMax))
  (bind _lightsflickeringtimermin (Variables|Default|GetLightsFlickeringTimerMin))
  (switch int (Math|Random|RandomInteger 3)
    (:0
      (CallFunction|Evento1 _lightsflickeringtimermin _lightsflickeringtimermax))
    (:1
      (CallFunction|Evento2 _lightsflickeringtimermin _lightsflickeringtimermax))
    (:2
      (CallFunction|Evento3 :!label _label))
    (:3
      (goto _label))))

(event Custom|Random%20Event%20Timer
  (Utilities|Time|SetTimerbyEvent (delegate Custom|EventosAleatorios%20-%20Selector) (Math|Random|RandomFloatinRange (Variables|Default|GetMinTimeToAction) (Variables|Default|GetMaxTimeToAction%20)) true))

(event EventBeginPlay
  (Audio|PlaySound2D "/Game/Audio/RandomUnderwaterLoop.RandomUnderwaterLoop" 1.0 1.0 0.0 0 0)
  (bind _returnvalue (Game|GetCurrentLevelName true))
  (if (not (Math|Boolean|ORBoolean (Utilities|Enum|Equal(Enum) _returnvalue "Tutorial") (Utilities|Enum|Equal(Enum) _returnvalue "Level4") (Utilities|Enum|Equal(Enum) _returnvalue "Checkpoint")))
    (CallFunction|RandomEventTimer)))

(event EventDerrota
  (|PantallaDerrota))

(event Custom|Evento1
  (params (Min :type Float%20%28double-precision%29) (Max :type Float%20%28double-precision%29))
  (bind _returnvalue (Math|Random|RandomFloatinRange Min Max))
  (bind _returnvalue_2 (+ _returnvalue 5.0))
  ;[1 1 1] Luces
  (Default|CallFlickeringLightsEvent _returnvalue)
  (Utilities|FlowControl|Delay _returnvalue_2)
  ;[1 1 1] Sonido Monstruo
  (Default|CallMonsterSoundsPlayEvent)
  (Utilities|FlowControl|Delay (+ _returnvalue_2 5.0))
  (Default|CallResetMainLights)
  (Audio|PlaySound2D "/Game/Audio/LightsBack.LightsBack" 1.0 1.0 0.0 0 0))

(event Custom|Evento2
  (params (Min :type Float%20%28double-precision%29) (Max :type Float%20%28double-precision%29))
  (bind _returnvalue (Math|Random|RandomFloatinRange Min Max))
  ;[1 1 1] Luces
  (Default|CallFlickeringLightsEvent _returnvalue)
  (Utilities|FlowControl|Delay (+ _returnvalue 5.0))
  (Default|CallResetMainLights)
  (Audio|PlaySound2D "/Game/Audio/LightsBack.LightsBack" 1.0 1.0 0.0 0 0))

(event Custom|Evento3
  (Audio|PlaySound2D "/Game/Audio/RandomEventSound_Cue.RandomEventSound_Cue" 1.0 1.0 0.0 0 0))

(event Custom|Evento%20Ataque
  (bind _returnvalue (Math|Random|RandomFloatinRange 5.0 1e+01))
  (bind _returnvalue_2 (+ _returnvalue 2.5))
  (Default|CallWaterFlowEvent)
  (CallFunction|RandomRuptura)
  (Default|CallFlickeringLightsEvent _returnvalue)
  (Default|CallImpactEvent)
  (Default|CallAlarmEvent)
  (Audio|PlaySound2D "/Game/Audio/Impact1.Impact1" 1.0 1.0 0.0 0 0)
  (Audio|PlaySound2D "/Game/Audio/Alarm.Alarm" 1.0 1.0 0.0 0 0)
  (Utilities|FlowControl|Delay _returnvalue_2)
  (Default|CallMonsterSoundsPlayEvent)
  (Utilities|FlowControl|Delay (+ _returnvalue_2 2.5))
  (Default|CallResetMainLights))

(event Custom|RandomRuptura
  (switch int (Math|Random|RandomInteger 2)
    (:0
      (Default|CallMotorBreakEvent))
    (:1
      (Default|CallOxygenBreakEvent))
    (:2
      (Default|CallMotorBreakEvent)
      (Default|CallOxygenBreakEvent))))

(fn ConstructionScript)