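; Spawner actor that creates BP_Coleccionable pickups at BeginPlay, choosing which collectibles appear based on the current level.
; The Tutorial gets one at a fixed position; other levels derive an index range from the level-name digit and spawn at random points within Box.
; Configuration macros fill name, description, mesh and material from parallel arrays and enlarge each pickup, which is then attached to BP_MovimientoMapa.
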(event Custom|SpawnColeccionables
  (bind _box (Variables|Default|GetBox))
  (bind _returnvalue (Game|GetCurrentLevelName true))
  (if (Utilities|Enum|Equal(Enum) _returnvalue "Tutorial")
    (bind _returnvalue_2 (Actor|GetActorOfClass "/Game/Blueprints/Objetos/V2/BP_MovimientoMapa.BP_MovimientoMapa_C"))
    (for _index (range 0 0)
      (bind _returnvalue_3 (Game|SpawnActorfromClass "/Game/Blueprints/Objetos/V2/BP_Coleccionable.BP_Coleccionable_C" (Math|Transform|MakeTransform "0.000000,-400.000000,124.000000" "0, 0, 0" "1.000000,1.000000,1.000000") "AdjustIfPossibleButAlwaysSpawn" "MultiplyWithRoot" 0 0))
      (|ConfigurarObjeto_2 _index _returnvalue_3)
      (Transformation|AttachActorToActor _returnvalue_3 _returnvalue_2 "None" "KeepWorld" "KeepWorld" "KeepWorld" false)
      (Development|PrintString (Utilities|String|ToString(Integer) _index) true true "(R=0.000000,G=1.000000,B=0.809316,A=1.000000)"))
    (Development|PrintString "Done" true true "(R=1.000000,G=0.014359,B=0.000000,A=1.000000)")
    (else
      (|ObjetosSegunNivel
        (:then
          _)
        (:then2
          _)
        (:then3
          _))
      (bind _returnvalue_4 (Actor|GetActorOfClass "/Game/Blueprints/Objetos/V2/BP_MovimientoMapa.BP_MovimientoMapa_C"))
      (for _index_2 (range (Variables|Default|GetIndiceInicial) (Variables|Default|GetIndiceFinal))
        (bind _returnvalue_5 (Game|SpawnActorfromClass "/Game/Blueprints/Objetos/V2/BP_Coleccionable.BP_Coleccionable_C" (Math|Transform|MakeTransform (Math|Random|RandomPointinBoundingBox (Transformation|GetWorldLocation _box) (Variables|/Script/Engine.BoxComponent|GetBoxExtent _box)) "0, 0, 0" "1.000000,1.000000,1.000000") "AdjustIfPossibleButAlwaysSpawn" "MultiplyWithRoot" 0 0))
        (|ConfigurarObjeto _index_2 _returnvalue_5)
        (Transformation|AttachActorToActor _returnvalue_5 _returnvalue_4 "None" "KeepWorld" "KeepWorld" "KeepWorld" false)
        (Development|PrintString (Utilities|String|ToString(Integer) _index_2) true true "(R=0.000000,G=1.000000,B=0.809316,A=1.000000)"))
      (Development|PrintString "Done" true true "(R=1.000000,G=0.014359,B=0.000000,A=1.000000)"))))

(event EventBeginPlay
  (CallFunction|SpawnColeccionables))

(fn ConstructionScript)