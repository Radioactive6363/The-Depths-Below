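; BP_Monstruo is the monster character, exposing events for its attack, sound, movement speed and sonar interaction.
; On BeginPlay it finds the BP_SonarV2 actor in the level and gets the game mode.
; Its events act as thin relays, triggering EventoAtaque on the game mode and SonarPingMessage on the sonar.
; Others play a monster sound or set the max fly speed.
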(event Custom|PlayMonsterSounds
  (bind _audio (Variables|Default|GetAudio))
  (Audio|Components|Audio|SetSound _audio "/Game/Audio/MonsterAudio1.MonsterAudio1")
  (Audio|Components|Audio|Play _audio 0.0))

(event EventSendMonsterSpeed
  (params (Float :type Float%20%28double-precision%29))
  (Variables|/Script/Engine.CharacterMovementComponent|SetMaxFlySpeed (Variables|Character|GetCharacterMovement) Float))

(event EventBeginPlay
  (Utilities|FlowControl|Sequence
    (:then_0
      (bind _returnvalue (Actor|GetActorOfClass "/Game/Blueprints/Objetos/V2/BP_SonarV2.BP_SonarV2_C"))
      (Variables|Default|SetSonar _returnvalue))
    (:then_1
      (bind _gamemode (Utilities|GetGameMode)))))

(event EventCallEvents
  (Default|EventoAtaque (stale EventBeginPlay _gamemode)))

(event EventCallSonar
  (Class|BPISonarPing|SonarPing(Message) (Variables|Default|GetSonar)))

(fn ConstructionScript)