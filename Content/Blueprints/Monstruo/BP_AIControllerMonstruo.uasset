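; AI controller for the monster, which runs the BT_Monstruo behavior tree against the player's submarine.
; On BeginPlay it seeds the blackboard with the BP_Submarino actor, minimum and maximum distances, a cleared detection flag and zeroed detection probabilities.
; Two custom events write incoming horizontal and vertical navigation detection probabilities to the blackboard.
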(event Custom|ProbDeteccionHor_1
  (params (DeteccionHor :type Float%20%28double-precision%29))
  (AI|Components|Blackboard|SetValueasFloat (AI|GetBlackboard 0) (Variables|Default|GetProbNavegacionDetHor) DeteccionHor))

(event EventBeginPlay
  (bind _returnvalue (AI|GetBlackboard 0))
  (AI|RunBehaviorTree "/Game/Blueprints/Monstruo/BT_Monstruo.BT_Monstruo")
  (Utilities|FlowControl|Sequence
    (:then_0
      (bind _returnvalue_2 (Actor|GetActorOfClass "/Game/Blueprints/Objetos/V2/BP_Submarino.BP_Submarino_C"))
      (AI|Components|Blackboard|SetValueasObject _returnvalue (Variables|Default|GetSubmarino/Player) _returnvalue_2))
    (:then_1
      (AI|Components|Blackboard|SetValueasFloat _returnvalue (Variables|Default|GetDistanciaMaxima) 3e+03))
    (:then_2
      (AI|Components|Blackboard|SetValueasFloat _returnvalue (Variables|Default|GetDistanciaMinima) 1e+02))
    (:then_3
      (AI|Components|Blackboard|SetValueasBool _returnvalue (Variables|Default|GetDetected?) false))
    (:then_4
      (AI|Components|Blackboard|SetValueasFloat _returnvalue (Variables|Default|GetProbNavegacionDetHor) 0.0))
    (:then_5
      (AI|Components|Blackboard|SetValueasFloat _returnvalue (Variables|Default|GetProbNavegacionDetVer) 0.0))))

(event EventProbDeteccionVer
  (params (DeteccionVer :type Float%20%28double-precision%29))
  (AI|Components|Blackboard|SetValueasFloat (AI|GetBlackboard 0) (Variables|Default|GetProbNavegacionDetVer) DeteccionVer))

(fn ConstructionScript)