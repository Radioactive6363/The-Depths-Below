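; Horizontal navigation lever station for a submarine: interacting with its trigger switches camera and lets player input tilt the lever.
; Input maps to lever angles and clamped velocities, animated by a timeline and sent to BP_MovimientoMapa to move the sub.
; An off-center lever reports higher detection probability to the monster AI.
; Disabling it turns the LED red, exits the camera, recenters the lever and zeroes velocity.
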(event Custom|CambioDeCamara
  ;[0 0.3354 0.3802] Cambio de Camara
  (bind _isa (Utilities|CameraChange (Variables|Default|GetCamera)))
  (Variables|Test|SetActivo? _isa)
  (if (Variables|Default|GetTutoActive?)
    (Default|CallTutorialNavHorizontal)))

(event Custom|InutilizacionNavegacion
  (params (Utilizable? :type Boolean))
  ;[1 0 0] Inutilizacion Navegacion (Rotura/Motor Apagado)
  (bind _output_get (Variables|Test|SetUtilizable? Utilizable?))
  (Utilities|EncenderLuz _output_get)
  (Utilities|FlowControl|Sequence
    (:then_0
      (if (Variables|Test|GetActivo?)
        (CallFunction|CambioDeCamara)))
    (:then_1
      (CallFunction|Desactivacion))))

(event Custom|Desactivacion
  ;[1 0 0] Inutilizacion Navegacion (Rotura/Motor Apagado)
  (Audio|Components|Audio|Stop (Variables|Default|GetMovimientoPalancaHorizontal))
  (bind _rotationalpha (Timeline|Timeline PlayFromStart)
    (:Update
      (Transformation|SetRelativeRotation (Variables|Default|GetPalancaMesh) (Math|Rotator|MakeRotator (Math|Float|Lerp (.x (Variables|Test|GetPalancaAnguloActual)) 0.0 _rotationalpha) (Math|Float|Lerp (.y (Variables|Test|GetPalancaAnguloActual)) 0.0 _rotationalpha) 0.0) false false))
    (:Finished
      (bind _output_get (Variables|Test|SetVelocidadActual ""))
      (CallFunction|EnviarVelocidadActual (.x _output_get) (.y _output_get))
      (Variables|Test|SetPalancaAnguloActual (Math|Vector2D|MakeVector2D (Math|Float|Lerp (.x (Variables|Test|GetPalancaAnguloActual)) 0.0 _rotationalpha) (Math|Float|Lerp (.y (Variables|Test|GetPalancaAnguloActual)) 0.0 _rotationalpha))))))

(event Custom|ResetNavegation
  ;[1 1 1] Reseteo de Valores Iniciales - Movimiento de Palanca (en caso de cambio del Valor del Index)
  ; Unicamente para Inicio y Testeo
  (Audio|Components|Audio|Stop (Variables|Default|GetMovimientoPalancaHorizontal))
  (bind _output_get (Variables|Test|SetPalancaAnguloActual ""))
  (Transformation|SetRelativeRotation (Variables|Default|GetPalancaMesh) (Math|Rotator|MakeRotator (.x _output_get) (.y _output_get) 0.0) false false)
  (bind _output_get_2 (Variables|Test|SetVelocidadActual ""))
  (CallFunction|EnviarVelocidadActual (.x _output_get_2) (.y _output_get_2))
  (Utilities|EncenderLuz (Variables|Test|GetUtilizable?)))

(event Custom|EnviarProbDeteccionHor
  (params (ProbDetHor :type Float%20%28double-precision%29))
  (Class|BPIDetNavegacionHor|ProbDeteccionHor(Message) (Variables|Default|GetIAMonstruo) ProbDetHor))

(event Custom|Enviar%20Velocidad%20Actual
  (params (VelocityX :type Float%20%28double-precision%29) (VelocityY :type Float%20%28double-precision%29))
  (Class|BPINavegacionHorizontal|MoverSubHorizontal(Message) (Variables|Default|GetMovimientoMapa) VelocityX VelocityY))

(event Custom|CambioVelocidad
  (params (InputValorX :type Float%20%28double-precision%29) (InputValorY :type Float%20%28double-precision%29))
  (bind (_anglex _angley _velocityx _velocityy) (|Velocidades InputValorX InputValorY))
  (bind _palancamesh (Variables|Default|GetPalancaMesh))
  (bind _returnvalue (Transformation|GetWorldRotation _palancamesh))
  ;[0.3802 0.1951 0.04189] Cambio de Velocidad - Animacion
  (if (Variables|Test|GetActivo?) ; True = Player en Navegacion\nFalse = Player NO esta en Navegacion
    (Variables|Test|SetPalancaAnguloActual (Math|Vector2D|MakeVector2D (.roll _returnvalue) (.pitch _returnvalue)))
    (bind _rotationalpha (Timeline|MovimientoPalancaHorizontal PlayFromStart)
      (:Update
        (Transformation|SetRelativeRotation (Variables|Default|GetPalancaMesh) (Math|Rotator|MakeRotator (Math|Float|Lerp (.x (Variables|Test|GetPalancaAnguloActual)) _anglex _rotationalpha) (Math|Float|Lerp (.y (Variables|Test|GetPalancaAnguloActual)) _angley _rotationalpha) 0.0) false false)
        (CallFunction|EnviarVelocidadActual _velocityx _velocityy))
      (:Finished
        (bind _output_get (Variables|Test|SetPalancaAnguloActual (Math|Vector2D|MakeVector2D (Math|Float|Lerp (.x (Variables|Test|GetPalancaAnguloActual)) _anglex _rotationalpha) (Math|Float|Lerp (.y (Variables|Test|GetPalancaAnguloActual)) _angley _rotationalpha))))))
    (if (Utilities|Operators|EqualEqual :B _output_get)
      (bind _output_get_2 (Variables|Default|SetProbDeteccionActual 0.0))
      (CallFunction|EnviarProbDeteccionHor _output_get_2)
      (else
        (bind _output_get_3 (Variables|Default|SetProbDeteccionActual 2e+01))
        (CallFunction|EnviarProbDeteccionHor _output_get_3)))))

(event Event4InputSystem
  (params (FloatX :type Float%20%28double-precision%29) (FloatY :type Float%20%28double-precision%29))
  ;[1 0.3471 0.9571] Evento Con Input - Cambio de Velocidad
  (CallFunction|CambioVelocidad FloatX FloatY))

(event EventObjectInteractions
  (params (SceneComponentTarget :type Scene%20Component%20Object%20Reference))
  ;[0.9471 0.4638 1] Interaccion con Objeto - Cambio de Camara
  (if (== SceneComponentTarget (Variables|Default|GetPalancaTrigger))
    (if (Variables|Test|GetUtilizable?) ; True = Llave Termica Encendida/Motor NO Roto\nFalse =  Llave Termica Apagada/Motor Roto
      (CallFunction|CambioDeCamara)
      (CallFunction|ResetNavegation)
      ;[0.3802 0.1951 0.04189] Cambio de Velocidad - Animacion
      (if (Utilities|Operators|EqualEqual :B (stale Custom|CambioVelocidad _output_get))
        (bind _output_get (Variables|Default|SetProbDeteccionActual 0.0))
        (CallFunction|EnviarProbDeteccionHor _output_get)
        (else
          (bind _output_get_2 (Variables|Default|SetProbDeteccionActual 2e+01))
          (CallFunction|EnviarProbDeteccionHor _output_get_2))))))

(event EventBeginPlay
  (Utilities|FlowControl|Sequence
    (:then_0
      (bind _returnvalue (Rendering|Material|CreateDynamicMaterialInstance "/Game/Materials/MI_Light.MI_Light" "None" "None" :!class /Script/Engine.KismetMaterialLibrary))
      (bind _output_get (Variables|Default|SetLuzMat _returnvalue))
      (Rendering|Material|SetMaterial (Variables|Default|GetLuzLed) 0 _output_get))
    (:then_1
      (CallFunction|ResetNavegation))
    (:then_2
      (bind _returnvalue_2 (Actor|GetActorOfClass "/Game/Blueprints/Objetos/V2/BP_MovimientoMapa.BP_MovimientoMapa_C"))
      (Variables|Default|SetMovimientoMapa _returnvalue_2))
    (:then_3
      (bind _returnvalue_3 (Actor|GetActorOfClass "/Game/Blueprints/Monstruo/BP_AIControllerMonstruo.BP_AIControllerMonstruo_C"))
      (Variables|Default|SetIAMonstruo _returnvalue_3))
    (:then_4
      (bind _returnvalue_4 (Game|GetCurrentLevelName true))
      (if (Utilities|Enum|Equal(Enum) _returnvalue_4 "Tutorial")
        (Variables|Default|SetTutoActive? true)))))

(event EventObjectActivate
  (params (Activate? :type Boolean))
  ;[1 0.3471 0.9571] Accion de Objeto - Inutilizacion Navegacion
  (CallFunction|InutilizacionNavegacion Activate?))

(fn ConstructionScript)

(fn GetAnglewithInputs
  (params (InputX :type Float%20%28double-precision%29) (InputY :type Float%20%28double-precision%29))
  (bind _palancaangulosmaximos (Variables|Test|GetPalancaAngulosMaximos))
  (return (Math|Float|MapRangeClamped (Math|Float|Clamp(Float) InputX -1.0) -1.0 1.0 (.y _palancaangulosmaximos) (.x _palancaangulosmaximos)) (Math|Float|MapRangeClamped (Math|Float|Clamp(Float) InputY -1.0) -1.0 1.0 (.x _palancaangulosmaximos) (.y _palancaangulosmaximos))))

(fn GetVelocitywithInputs
  (params (InputX :type Float%20%28double-precision%29) (InputY :type Float%20%28double-precision%29))
  (bind _velocidadmaxima (Variables|Test|GetVelocidadMaxima))
  (bind _output_get (Variables|Test|SetVelocidadActual (Math|Vector2D|MakeVector2D (Math|Float|MapRangeClamped (Math|Float|Clamp(Float) InputX -1.0) -1.0 1.0 (* _velocidadmaxima -1.0) _velocidadmaxima) (Math|Float|MapRangeClamped (Math|Float|Clamp(Float) InputY -1.0) -1.0 1.0 (* _velocidadmaxima -1.0) _velocidadmaxima))))
  (return (.x _output_get) (.y _output_get)))

(fn IsHoveringActor
  (params (Hit :type Hit%20Result%20Structure) (Player :type BP%20Personaje%20V2%20Object%20Reference))
  (if (Math|Boolean|ANDBoolean (== (Variables|Default|GetPalancaTrigger) (.HitComponent (Collision|BreakHitResult Hit))) (not (Variables|Test|GetActivo?)) (Variables|Test|GetUtilizable?))
    (return "Manejar")
    (else
      (return ""))))