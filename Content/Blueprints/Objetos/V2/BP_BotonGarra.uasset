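; Interactable button that runs a claw crane sequence, then tells the stored collectible reference to teleport to the hatch.
; Pressing it locks it, animates the button with a timeline, then chains the PickUp and Retract montages with crane audio before unlocking.
; A dynamic material shows green when available and red when locked; Inutilizacion sets the lock externally.
; In the Tutorial level, interactions also fire a tutorial call.
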(event Custom|BotonActivacionGarra
  (if (not (Variables|Default|GetDelayActivo?))
    (bind _output_get (Variables|Default|SetLocalizacionInicial (Variables|/Script/Engine.SceneComponent|GetRelativeLocation (Variables|Default|GetBoton))))
    (bind _output_get_2 (Variables|Default|SetDelayActivo? true))
    (Utilities|Encendido/ApagadoLuces _output_get_2)
    (Audio|PlaySoundatLocation "/Game/Audio/PushButton.PushButton" _output_get "0, 0, 0" 0.25 1.0 0.0 0 0 0 0)
    (bind _animacionboton (Timeline|MovimientoBoton PlayFromStart)
      (:Update
        (Transformation|SetRelativeLocation (Variables|Default|GetBoton) (Math|Vector|Lerp(Vector) (Variables|Default|GetLocalizacionInicial) (+ (Variables|Default|GetLocalizacionInicial) "0.000000,0.000000,-5.000000") _animacionboton) false false))
      (:Finished
        (CallFunction|AnimacionGarra)))))

(event Custom|AnimacionGarra
  (Animation|Montage|PlayMontage (Variables|Default|GetGarra) "/Game/Animations/AM_GarraAnimation.AM_GarraAnimation" 1.0 0.0 "PickUp"
    (:then
      (Audio|Components|Audio|Play (Variables|Default|GetCraneSound_Cue) 0.0))
    (:OnCompleted
      (Animation|Montage|PlayMontage (Variables|Default|GetGarra) "/Game/Animations/AM_GarraAnimation.AM_GarraAnimation" 1.0 2.1e+02 "Retract"
        (:OnCompleted
          (Audio|Components|Audio|Stop (Variables|Default|GetCraneSound_Cue))
          (Class|BPIColeccionableHaciaGarra|TeleporttoHatch(Message) (Variables|Default|GetColeccionableReference))
          (bind _output_get (Variables|Default|SetDelayActivo? false))
          (Utilities|Encendido/ApagadoLuces _output_get))))))

(event Custom|Inutilizacion
  (params (Delay? :type Boolean))
  (bind _output_get (Variables|Default|SetDelayActivo? Delay?))
  (Utilities|Encendido/ApagadoLuces _output_get))

(event EventBeginPlay
  (Utilities|FlowControl|Sequence
    (:then_0
      (bind _returnvalue (Rendering|Material|CreateDynamicMaterialInstance "/Game/Materials/MI_Light.MI_Light" "None" "None" :!class /Script/Engine.KismetMaterialLibrary))
      (bind _output_get (Variables|Default|SetLuzMat _returnvalue))
      (Rendering|Material|SetMaterial (Variables|Default|GetBoton) 0 _output_get))
    (:then_1
      (bind _returnvalue_2 (Game|GetCurrentLevelName true))
      (if (Utilities|Enum|Equal(Enum) _returnvalue_2 "Tutorial")
        (Variables|Default|SetTutoActive? true)))))

(event EventObjectCollectedReference
  (params (Coleccionable :type Actor%20Object%20Reference))
  (Variables|Default|SetColeccionableReference Coleccionable))

(event EventObjectInteractions
  (params (SceneComponentTarget :type Scene%20Component%20Object%20Reference))
  (CallFunction|BotonActivacionGarra)
  (if (Variables|Default|GetTutoActive?)
    (Default|CallTutorialButtonGarra)))

(fn ConstructionScript)