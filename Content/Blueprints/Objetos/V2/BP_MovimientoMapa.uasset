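; Map actor that simulates submarine navigation by moving the level, with velocities driving a self-restarting timeline and Niagara water particle speed.
; Tick increments game-instance depth as Trigger Z changes and feeds position and first point-of-interest coordinates to monitor widgets.
; Points of interest are collectibles and the black box, sorted by height.
; Submarine overlaps show collision screens and nudge the map back by quadrant; Level4's Ending stops vertical motion and activates horizontal navigation.
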(event OnComponentBeginOverlap(Ending)
  (params (OverlappedComponent :type Primitive%20Component%20Object%20Reference) (OtherActor :type Actor%20Object%20Reference) (OtherComp :type Primitive%20Component%20Object%20Reference) (OtherBodyIndex :type Integer) (bFromSweep :type Boolean) (SweepResult :type Hit%20Result%20Structure%20%28by%20ref%29))
  (bind _returnvalue (Game|GetCurrentLevelName true))
  (if (and (Utilities|Enum|Equal(Enum) _returnvalue "Level4") (Class|GameplayStatics|ObjectIsA OtherActor "/Game/Blueprints/Objetos/V2/BP_Submarino.BP_Submarino_C"))
    (Variables|Default|SetVelocidadActualZ 0.0)
    (CallFunction|AceleracionParticulas)
    (CallFunction|Aceleracion)
    (bind _returnvalue_2 (Actor|GetActorOfClass "/Game/Blueprints/Objetos/V2/BP_LlaveTermica.BP_LlaveTermica_C"))
    (Default|ObjectActivate _returnvalue_2 false)
    (Utilities|FlowControl|Delay 1.0)
    (bind _returnvalue_3 (Actor|GetActorOfClass "/Game/Blueprints/Objetos/V2/BP_NavegacionHorizontal.BP_NavegacionHorizontal_C"))
    (Default|ObjectActivate _returnvalue_3 true)))

(event OnComponentBeginOverlap(Mapa)
  (params (OverlappedComponent :type Primitive%20Component%20Object%20Reference) (OtherActor :type Actor%20Object%20Reference) (OtherComp :type Primitive%20Component%20Object%20Reference) (OtherBodyIndex :type Integer) (bFromSweep :type Boolean) (SweepResult :type Hit%20Result%20Structure%20%28by%20ref%29))
  (bind _returnvalue (Transformation|GetActorLocation))
  (Development|PrintString (Utilities|GetDisplayName OtherActor))
  (if (== (Utilities|GetClass OtherActor) "/Game/Blueprints/Objetos/V2/BP_Submarino.BP_Submarino_C")
    (Variables|Default|SetcolX (.x _returnvalue))
    (Variables|Default|SetcolY (.y _returnvalue))
    (if (and (< (.x _returnvalue) 0.0) (< (.y _returnvalue) 0.0))
      (bind _returnvalue_2 (Actor|GetActorOfClass "/Game/Blueprints/Objetos/V2/BP_MonitorHorizontal.BP_MonitorHorizontal_C"))
      (bind _asbp_monitor_horizontal_ui (Utilities|Casting|CastToBP_MonitorHorizontalUI (UserInterface|GetWidget (Variables|/Game/Blueprints/Objetos/V2/BP_MonitorHorizontal.BP_MonitorHorizontal_C|GetMonitorHorizontalUI _returnvalue_2))))
      (Widget|SetVisibility (Variables|/Game/Blueprints/UI/Objetos/V2/BP_MonitorHorizontalUI.BP_MonitorHorizontalUI_C|GetPantallaInicial _asbp_monitor_horizontal_ui) "Hidden")
      (Widget|SetVisibility (Variables|/Game/Blueprints/UI/Objetos/V2/BP_MonitorHorizontalUI.BP_MonitorHorizontalUI_C|GetColision _asbp_monitor_horizontal_ui) "Visible")
      (bind _returnvalue_3 (Actor|GetActorOfClass "/Game/Blueprints/Objetos/V2/BP_MonitorProfActual.BP_MonitorProfActual_C"))
      (bind _asbp_prof_actual_ui (Utilities|Casting|CastToBP_ProfActualUI (UserInterface|GetWidget (Variables|/Game/Blueprints/Objetos/V2/BP_MonitorProfActual.BP_MonitorProfActual_C|GetProfActualUI _returnvalue_3))))
      (Widget|SetVisibility (Variables|/Game/Blueprints/UI/Objetos/V2/BP_ProfActualUI.BP_ProfActualUI_C|GetPantallaInicial _asbp_prof_actual_ui) "Hidden")
      (Widget|SetVisibility (Variables|/Game/Blueprints/UI/Objetos/V2/BP_ProfActualUI.BP_ProfActualUI_C|GetColision _asbp_prof_actual_ui) "Visible")
      (|Correccion)
      (elif (and (>= (.x _returnvalue) 0.0) (<= (.y _returnvalue) 0.0))
        (bind _returnvalue_4 (Actor|GetActorOfClass "/Game/Blueprints/Objetos/V2/BP_MonitorHorizontal.BP_MonitorHorizontal_C"))
        (bind _asbp_monitor_horizontal_ui_2 (Utilities|Casting|CastToBP_MonitorHorizontalUI (UserInterface|GetWidget (Variables|/Game/Blueprints/Objetos/V2/BP_MonitorHorizontal.BP_MonitorHorizontal_C|GetMonitorHorizontalUI _returnvalue_4))))
        (Widget|SetVisibility (Variables|/Game/Blueprints/UI/Objetos/V2/BP_MonitorHorizontalUI.BP_MonitorHorizontalUI_C|GetPantallaInicial _asbp_monitor_horizontal_ui_2) "Hidden")
        (Widget|SetVisibility (Variables|/Game/Blueprints/UI/Objetos/V2/BP_MonitorHorizontalUI.BP_MonitorHorizontalUI_C|GetColision _asbp_monitor_horizontal_ui_2) "Visible")
        (bind _returnvalue_5 (Actor|GetActorOfClass "/Game/Blueprints/Objetos/V2/BP_MonitorProfActual.BP_MonitorProfActual_C"))
        (bind _asbp_prof_actual_ui_2 (Utilities|Casting|CastToBP_ProfActualUI (UserInterface|GetWidget (Variables|/Game/Blueprints/Objetos/V2/BP_MonitorProfActual.BP_MonitorProfActual_C|GetProfActualUI _returnvalue_5))))
        (Widget|SetVisibility (Variables|/Game/Blueprints/UI/Objetos/V2/BP_ProfActualUI.BP_ProfActualUI_C|GetPantallaInicial _asbp_prof_actual_ui_2) "Hidden")
        (Widget|SetVisibility (Variables|/Game/Blueprints/UI/Objetos/V2/BP_ProfActualUI.BP_ProfActualUI_C|GetColision _asbp_prof_actual_ui_2) "Visible")
        (|Correccion2)
        (elif (and (<= (.x _returnvalue) 0.0) (>= (.y _returnvalue) 0.0))
          (bind _returnvalue_6 (Actor|GetActorOfClass "/Game/Blueprints/Objetos/V2/BP_MonitorHorizontal.BP_MonitorHorizontal_C"))
          (bind _asbp_monitor_horizontal_ui_3 (Utilities|Casting|CastToBP_MonitorHorizontalUI (UserInterface|GetWidget (Variables|/Game/Blueprints/Objetos/V2/BP_MonitorHorizontal.BP_MonitorHorizontal_C|GetMonitorHorizontalUI _returnvalue_6))))
          (Widget|SetVisibility (Variables|/Game/Blueprints/UI/Objetos/V2/BP_MonitorHorizontalUI.BP_MonitorHorizontalUI_C|GetPantallaInicial _asbp_monitor_horizontal_ui_3) "Hidden")
          (Widget|SetVisibility (Variables|/Game/Blueprints/UI/Objetos/V2/BP_MonitorHorizontalUI.BP_MonitorHorizontalUI_C|GetColision _asbp_monitor_horizontal_ui_3) "Visible")
          (bind _returnvalue_7 (Actor|GetActorOfClass "/Game/Blueprints/Objetos/V2/BP_MonitorProfActual.BP_MonitorProfActual_C"))
          (bind _asbp_prof_actual_ui_3 (Utilities|Casting|CastToBP_ProfActualUI (UserInterface|GetWidget (Variables|/Game/Blueprints/Objetos/V2/BP_MonitorProfActual.BP_MonitorProfActual_C|GetProfActualUI _returnvalue_7))))
          (Widget|SetVisibility (Variables|/Game/Blueprints/UI/Objetos/V2/BP_ProfActualUI.BP_ProfActualUI_C|GetPantallaInicial _asbp_prof_actual_ui_3) "Hidden")
          (Widget|SetVisibility (Variables|/Game/Blueprints/UI/Objetos/V2/BP_ProfActualUI.BP_ProfActualUI_C|GetColision _asbp_prof_actual_ui_3) "Visible")
          (|Correccion3)
          (elif (and (> (.x _returnvalue) 0.0) (> (.y _returnvalue) 0.0))
            (bind _returnvalue_8 (Actor|GetActorOfClass "/Game/Blueprints/Objetos/V2/BP_MonitorHorizontal.BP_MonitorHorizontal_C"))
            (bind _asbp_monitor_horizontal_ui_4 (Utilities|Casting|CastToBP_MonitorHorizontalUI (UserInterface|GetWidget (Variables|/Game/Blueprints/Objetos/V2/BP_MonitorHorizontal.BP_MonitorHorizontal_C|GetMonitorHorizontalUI _returnvalue_8))))
            (Widget|SetVisibility (Variables|/Game/Blueprints/UI/Objetos/V2/BP_MonitorHorizontalUI.BP_MonitorHorizontalUI_C|GetPantallaInicial _asbp_monitor_horizontal_ui_4) "Hidden")
            (Widget|SetVisibility (Variables|/Game/Blueprints/UI/Objetos/V2/BP_MonitorHorizontalUI.BP_MonitorHorizontalUI_C|GetColision _asbp_monitor_horizontal_ui_4) "Visible")
            (bind _returnvalue_9 (Actor|GetActorOfClass "/Game/Blueprints/Objetos/V2/BP_MonitorProfActual.BP_MonitorProfActual_C"))
            (bind _asbp_prof_actual_ui_4 (Utilities|Casting|CastToBP_ProfActualUI (UserInterface|GetWidget (Variables|/Game/Blueprints/Objetos/V2/BP_MonitorProfActual.BP_MonitorProfActual_C|GetProfActualUI _returnvalue_9))))
            (Widget|SetVisibility (Variables|/Game/Blueprints/UI/Objetos/V2/BP_ProfActualUI.BP_ProfActualUI_C|GetPantallaInicial _asbp_prof_actual_ui_4) "Hidden")
            (Widget|SetVisibility (Variables|/Game/Blueprints/UI/Objetos/V2/BP_ProfActualUI.BP_ProfActualUI_C|GetColision _asbp_prof_actual_ui_4) "Visible")
            (|Correccion4)))))))

(event Custom|Aceleracion
  ;[1 1 1] Aceleracion del Movimiento
  (if (not (and (and (== (Variables|Default|GetVelocidadActualX) 0.0) (== (Variables|Default|GetVelocidadActualY) 0.0)) (== (Variables|Default|GetVelocidadActualZ) 0.0)))
    (Variables|Default|SetPosicionActual (Transformation|GetActorLocation))
    (bind _moversubmarino (Timeline|BaseTimeline PlayFromStart)
      (:Update
        (Transformation|SetActorRelativeLocation (Math|Vector|Lerp(Vector) (Math|Vector|MakeVector (.x (Variables|Default|GetPosicionActual)) (.y (Variables|Default|GetPosicionActual)) (.z (Variables|Default|GetPosicionActual))) (+ (Math|Vector|MakeVector (* (Variables|Default|GetVelocidadActualX) 1e+01) (* (Variables|Default|GetVelocidadActualY) 1e+01) (* (Variables|Default|GetVelocidadActualZ) 1e+01)) (Math|Vector|MakeVector (.x (Variables|Default|GetPosicionActual)) (.y (Variables|Default|GetPosicionActual)) (.z (Variables|Default|GetPosicionActual)))) _moversubmarino)))
      (:Finished
        (Variables|Default|SetPosicionActual (Transformation|GetActorLocation))
        (CallFunction|Aceleracion)))))

(event Custom|Aceleracion%20Particulas
  (bind (_velocidadparticulas _velocidad___0) (CallFunction|VelocidadDeParticulas))
  (bind _waterparticles (Variables|Default|GetWaterParticles))
  (bind _niagaracomponent (Variables|/Script/Niagara.NiagaraActor|GetNiagaraComponent _waterparticles))
  ;[1 1 1] Aceleracion de las Particulas
  (if _velocidad___0
    (Effects|Components|ParticleSystem|SetVectorParameter _niagaracomponent "User.ParticleSpeed" (Variables|Default|GetVelocidadDefaultParticulas))
    (else
      (Effects|Components|ParticleSystem|SetVectorParameter _niagaracomponent "User.ParticleSpeed" _velocidadparticulas))))

(event Custom|Actualizar%20Profundidad
  (bind _trigger (Variables|Default|GetTrigger))
  (bind _returnvalue (Transformation|GetWorldLocation _trigger))
  (bind _returnvalue_2 (Math|Float|Truncate (.z _returnvalue)))
  ;[1 1 1] Actualizar Profundidad
  (if (and (!= (Variables|Default|GetPosPrevia) _returnvalue_2) (< _returnvalue_2 0))
    (Variables|Default|SetPosPrevia _returnvalue_2)
    (bind _asbp_instance (Utilities|Casting|CastToBP_Instance (Game|GetGameInstance)))
    (Variables|/Game/Blueprints/BP_Instance.BP_Instance_C|SetProf _asbp_instance (+ (Variables|/Game/Blueprints/BP_Instance.BP_Instance_C|GetProf _asbp_instance) 1))))

(event Custom|PosicionHorizontal
  (bind _returnvalue (Transformation|GetActorLocation))
  ;[1 1 1] PosiciónHorizontal
  (bind _returnvalue_2 (Actor|GetActorOfClass "/Game/Blueprints/Objetos/V2/BP_MonitorHorizontal.BP_MonitorHorizontal_C"))
  (bind _asbp_monitor_horizontal_ui (Utilities|Casting|CastToBP_MonitorHorizontalUI (UserInterface|GetWidget (Variables|/Game/Blueprints/Objetos/V2/BP_MonitorHorizontal.BP_MonitorHorizontal_C|GetMonitorHorizontalUI _returnvalue_2))))
  (Variables|/Game/Blueprints/UI/Objetos/V2/BP_MonitorHorizontalUI.BP_MonitorHorizontalUI_C|SetMovX _asbp_monitor_horizontal_ui (Math|Float|Truncate (.x _returnvalue)))
  (Variables|/Game/Blueprints/UI/Objetos/V2/BP_MonitorHorizontalUI.BP_MonitorHorizontalUI_C|SetMovY _asbp_monitor_horizontal_ui (Math|Float|Truncate (.y _returnvalue))))

(event Custom|GetPuntoInteres
  (bind _actorcolecref (Variables|Default|GetActorColecRef))
  (bind _outactors (Actor|GetAllActorsOfClass "/Game/Blueprints/Objetos/V2/BP_Coleccionable.BP_Coleccionable_C"))
  (for _array_element _outactors
    (Utilities|IsValid _array_element
      (:Is%20Valid
        (Utilities|Array|Add (Variables|Default|GetActorColecRef) _array_element))))
  (bind _returnvalue (Actor|GetActorOfClass "/Game/Blueprints/Objetos/V2/BP_CajaNegra.BP_CajaNegra_C"))
  (Utilities|IsValid _returnvalue
    (:Is%20Valid
      (Utilities|Array|Add (Variables|Default|GetActorColecRef) _returnvalue)
      (for (_array_element_2 _array_index) _actorcolecref
        (for _index (range _array_index (- (Utilities|Array|Length _actorcolecref) 1))
          (if (> (.z (Transformation|GetWorldLocation (Variables|/Script/Engine.Actor|GetRootComponent (Utilities|Array|Get(acopy) (Variables|Default|GetActorColecRef) _index)))) (.z (Transformation|GetWorldLocation (Variables|/Script/Engine.Actor|GetRootComponent _array_element_2))))
            (Utilities|Array|Swap (Variables|Default|GetActorColecRef) _index _array_index))))
      (for _array_element_3 (Variables|Default|GetActorColecRef)
        (Utilities|Map|Add (Variables|Default|GetCoordenadasObjetos) (* (Math|Float|Truncate (.x (Transformation|GetWorldLocation (Variables|/Script/Engine.Actor|GetRootComponent _array_element_3)))) -1) (* (+ (Math|Float|Truncate (.y (Transformation|GetWorldLocation (Variables|/Script/Engine.Actor|GetRootComponent _array_element_3)))) 400) -1))))))

(event Custom|ResetChoque
  (Audio|Components|Audio|Stop (Variables|Default|GetBaseTimeline)))

(event Custom|PuntoInteresActual
  (bind _coordenadasobjetos (Variables|Default|GetCoordenadasObjetos))
  (bind _returnvalue (Actor|GetActorOfClass "/Game/Blueprints/Objetos/V2/BP_Camara.BP_Camara_C"))
  (bind _asbp_punto_interes (Utilities|Casting|CastToBP_PuntoInteres (UserInterface|GetWidget (Variables|/Game/Blueprints/Objetos/V2/BP_Camara.BP_Camara_C|GetCoordColecc _returnvalue))))
  (bind _keys (Utilities|Map|Keys _coordenadasobjetos))
  (bind _values (Utilities|Map|Values _coordenadasobjetos))
  (Variables|/Game/Blueprints/UI/Objetos/V2/BP_PuntoInteres.BP_PuntoInteres_C|SetMovX _asbp_punto_interes (Utilities|Array|Get(acopy) _keys))
  (Variables|/Game/Blueprints/UI/Objetos/V2/BP_PuntoInteres.BP_PuntoInteres_C|SetMovY _asbp_punto_interes (Utilities|Array|Get(acopy) _values)))

(event EventBeginPlay
  ;[1 1 1] Obtener Niagara Particles - Obtener Profundidad Del Nivel
  (Utilities|FlowControl|Sequence
    (:then_0
      (Variables|Default|SetPosPrevia (Math|Float|Truncate (.z (Transformation|GetWorldLocation (Variables|Default|GetTrigger))))))
    (:then_1
      (bind _returnvalue (Actor|GetActorOfClass "/Script/Niagara.NiagaraActor"))
      (Variables|Default|SetWaterParticles _returnvalue))
    (:then_2
      (Utilities|FlowControl|Delay 1.0)
      (CallFunction|GetPuntoInteres))))

(event EventMoverSubHorizontal
  (params (HorizontalX :type Float%20%28double-precision%29) (HorizontalY :type Float%20%28double-precision%29))
  ;[1 1 1] Obtener Velocidades Horizontales
  (Variables|Default|SetVelocidadActualX HorizontalX)
  (Variables|Default|SetVelocidadActualY HorizontalY)
  (CallFunction|AceleracionParticulas)
  (CallFunction|Aceleracion))

(event EventMoverSubVertical
  (params (VerticalZ :type Float%20%28double-precision%29))
  ;[1 1 1] Obtener Velocidades Verticales
  (Variables|Default|SetVelocidadActualZ VerticalZ)
  (CallFunction|AceleracionParticulas)
  (CallFunction|Aceleracion))

(event EventTick
  (params (DeltaSeconds :type Float%20%28single-precision%29))
  (CallFunction|ActualizarProfundidad)
  (CallFunction|PosicionHorizontal)
  (CallFunction|PuntoInteresActual))

(event EventMoverSubRotacion
  (params (RotacionZ :type Float%20%28double-precision%29))
  ;[1 1 1] Rotación
  (Transformation|SetActorRelativeRotation (Math|Rotator|MakeRotator 0.0 0.0 (+ (* RotacionZ -1.0) (.yaw (Transformation|GetActorRotation))))))

(fn ConstructionScript)

(fn VelocidadDeParticulas
  (bind _velocidadactualx (Variables|Default|GetVelocidadActualX))
  (bind _velocidadactualy (Variables|Default|GetVelocidadActualY))
  (bind _velocidadactualz (Variables|Default|GetVelocidadActualZ))
  (bind _returnvalue (Math|Float|MapRangeClamped _velocidadactualz 0.0 12.5 0.0 1.0))
  (bind _returnvalue_2 (Math|Float|MapRangeClamped _velocidadactualy -12.5 12.5 -1.0 1.0))
  (bind _returnvalue_3 (Math|Float|MapRangeClamped _velocidadactualx -12.5 12.5 -1.0 1.0))
  (bind _returnvalue_4 (* _returnvalue_2 1e+02))
  (bind _returnvalue_5 (* _returnvalue_3 1e+02))
  (bind _returnvalue_6 (* _returnvalue 1e+02))
  (bind _returnvalue_7 (Math|Vector|MakeVector _returnvalue_5 _returnvalue_4 _returnvalue_6))
  (return _returnvalue_7 (Utilities|Operators|EqualEqual :A _returnvalue_7)))