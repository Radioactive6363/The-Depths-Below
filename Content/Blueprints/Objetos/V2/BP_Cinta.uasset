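; BP_Cinta is an interactable "cinta" (tape) object, apparently meant to be grabbed and carried by the player.
; ObjectInteractions calls AgarradoDeCinta for the collision component, otherwise SoltarCinta, which clears the held flag, detaches and enables physics.
; The grab event is empty, with attach and move nodes left disconnected.
; LocalizacionCinta lerps the tape toward an offset from the player pawn with control rotation, but only unreachable code calls it.
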(event Custom|AgarradoDeCinta)

(event Custom|SoltarCinta
  (bind _output_get (Variables|Default|SetCintaAgarrada false))
  (Transformation|DetachFromActor "KeepRelative" "KeepRelative" "KeepRelative")
  (Physics|SetSimulatePhysics (Variables|Default|GetCinta) (not _output_get)))

(event EventObjectInteractions
  (params (SceneComponentTarget :type Scene%20Component%20Object%20Reference))
  (if (== SceneComponentTarget (Variables|Default|GetCintaCollision))
    (CallFunction|AgarradoDeCinta)
    (else
      (CallFunction|SoltarCinta))))

(fn ConstructionScript)