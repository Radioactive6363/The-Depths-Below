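; Base interactable submarine navigation lever that lets the player step through preset speeds, each with a monster detection probability.
; Hitting the lever trigger toggles a camera view while the lever is usable, and ObjectActivate sets that usability.
; In that view, input steps a clamped index and a timeline animates the lever with player input disabled.
; On finish, it passes speed and detection values to empty events that children override.
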(event Custom|CambioDeCamara
  ;[0 0.3354 0.3802] Cambio de Camara
  (bind _isa (Utilities|CameraChange (Variables|Default|GetCamera)))
  (Variables|Test|SetActivo? _isa))

(event Custom|CambioVelocidad
  (params (InputValor :type Float%20%28double-precision%29))
  ;[0.3802 0.1951 0.04189] Cambio de Velocidad - Animacion
  (if (Variables|Test|GetActivo?) ; True = Player en Navegacion\nFalse = Player NO esta en Navegacion
    (Utilities|InputPositivo/Negativo InputValor
      (:Input1
        (bind _outputindex (Utilities|Aumento/DisminucionIndex (Variables|Test|GetVelocidadesIndex) (- (Utilities|Array|Length (Variables|Test|GetVelocidades)) 1) :!label _label)
          (:Output1
            ;;[1 1 1] Movimiento Palanca - Animacion
            (bind _palancafloat (Timeline|MovimientoDePalanca PlayFromStart)
              (:Update
                (Input|DisableInput (Game|GetPlayerCharacter 0) (Game|GetPlayerController 0))
                (Transformation|SetRelativeRotation (Variables|Default|GetPalanca) (Math|Rotator|MakeRotator 0.0 (.y (Math|Vector|Lerp(Vector) (Math|Vector|MakeVector 0.0 (Variables|Test|GetAnguloPalancaActual) 0.0) (Math|Vector|MakeVector 0.0 (Utilities|Array|Get(acopy) (Variables|Test|GetAngulosPalanca) _outputindex) 0.0) _palancafloat)) 0.0) false false))
              (:Finished
                (Variables|Test|SetAnguloPalancaActual (Utilities|Array|Get(acopy) (Variables|Test|GetAngulosPalanca) (Variables|Test|GetVelocidadesIndex))) ; Actualizacion del Angulo de la Palanca
                (Input|EnableInput (Game|GetPlayerCharacter 0) (Game|GetPlayerController 0))
                (bind _output_get (Variables|Test|SetVelocidadActual (Utilities|Array|Get(acopy) (Variables|Test|GetVelocidades) (Variables|Test|GetVelocidadesIndex))))
                (CallFunction|EnviarVelocidadActual _output_get)
                (CallFunction|EnviarProbDeteccion (Utilities|Array|Get(acopy) (Variables|Test|GetProbabilidadDeteccion) (Variables|Test|GetVelocidadesIndex))))))
          (:Output2
            (Timeline|MovimientoDePalanca PlayFromStart))))
      (:Input2
        (goto _label Input2)))))

(event Custom|InutilizacionNavegacion
  (params (Utilizable? :type Boolean))
  ;[1 0 0] Inutilizacion Navegacion (Rotura/Motor Apagado)
  (Variables|Test|SetUtilizable? Utilizable?))

(event Custom|ResetNavegation
  (bind _angulospalanca (Variables|Test|GetAngulosPalanca))
  (bind _velocidadesindex (Variables|Test|GetVelocidadesIndex))
  (bind _output (Utilities|Array|Get(acopy) _angulospalanca _velocidadesindex))
  ;[1 1 1] Reseteo de Valores Iniciales - Movimiento de Palanca (en caso de cambio del Valor del Index)
  ; Unicamente para Inicio y Testeo
  (Transformation|SetRelativeRotation (Variables|Default|GetPalanca) (Math|Rotator|MakeRotator 0.0 _output 0.0) false false)
  (Variables|Test|SetAnguloPalancaActual _output))

(event Custom|EnviarProbDeteccion
  (params (ProbDeteccion :type Float%20%28double-precision%29))
  ;[1 1 1] NO ELIMINAR - Se hace Override en los "Children"
)

(event Custom|EnviarVelocidadActual
  (params (VelocidadActual :type Float%20%28double-precision%29))
  ;[1 1 1] NO ELIMINAR - Se hace Override en los "Children"
)

(event EventObjectW/Input
  (params (InputValor :type Float%20%28double-precision%29))
  ;[1 0.3471 0.9571] Evento Con Input - Cambio de Velocidad
  (CallFunction|CambioVelocidad InputValor))

(event EventObjectInteractions
  (params (SceneComponentTarget :type Scene%20Component%20Object%20Reference))
  ;[0.9471 0.4638 1] Interaccion con Objeto - Cambio de Camara
  (if (== SceneComponentTarget (Variables|Default|GetPalancaTrigger))
    (if (Variables|Test|GetUtilizable?) ; True = Llave Termica Encendida/Motor NO Roto\nFalse =  Llave Termica Apagada/Motor Roto
      (CallFunction|CambioDeCamara))))

(event EventBeginPlay
  (Utilities|FlowControl|Sequence
    (:then_0
      (CallFunction|ResetNavegation))
    (:then_1
      (bind _returnvalue (Actor|GetActorOfClass "/Game/Blueprints/Objetos/V2/SubmarinoTest.SubmarinoTest_C"))
      (Variables|Default|SetSubmarinoActor _returnvalue))
    (:then_2
      (bind _returnvalue_2 (Actor|GetActorOfClass "/Game/Blueprints/Monstruo/BP_AIControllerMonstruo.BP_AIControllerMonstruo_C"))
      (Variables|Default|SetIAMonstruo _returnvalue_2))))

(event EventObjectActivate
  (params (Activate? :type Boolean))
  ;[1 0.3471 0.9571] Accion de Objeto - Inutilizacion Navegacion
  (CallFunction|InutilizacionNavegacion Activate?))

(fn ConstructionScript)