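; Interactable digital terminal that shows a resource console UI on a widget component, with a hover prompt on its screen.
; On BeginPlay it picks the checkpoint or standard console widget based on the current level name.
; Interaction triggers a camera change that notifies the widget and switches between UI-only input with keyboard focus and game-only input.
; While active, Tick pins the mouse cursor to the viewport center.
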(event Custom|Cambio%20de%20Camara
  (bind _terminaldigitalui (Variables|Default|GetTerminalDigitalUI))
  (bind _returnvalue (UserInterface|GetWidget _terminaldigitalui))
  ;[0 0.3354 0.3802] Cambio de Camara
  (bind _isa (Utilities|CameraChange (Variables|Default|GetCamera)))
  (Variables|Default|SetActivo? _isa)
  (if _isa
    (Class|BPIInteractions|ObjectActivate(Message) _returnvalue _isa)
    (|FocusUI)
    (else
      (Class|BPIInteractions|ObjectActivate(Message) _returnvalue _isa)
      (|FocusGame))))

(event EventTick
  (params (DeltaSeconds :type Float%20%28single-precision%29))
  (if (Variables|Default|GetActivo?)
    (|MousealMediodelaPantalla)))

(event EventBeginPlay
  (|EleccionWidgetUI))

(event EventObjectInteractions
  (params (SceneComponentTarget :type Scene%20Component%20Object%20Reference))
  (CallFunction|CambioDeCamara))

(fn ConstructionScript)

(fn IsHoveringActor
  (params (Hit :type Hit%20Result%20Structure) (Player :type BP%20Personaje%20V2%20Object%20Reference))
  (if (and (== (Variables|Default|GetPantalla) (.HitComponent (Collision|BreakHitResult Hit))) (not (Variables|Default|GetActivo?)))
    (return "Acceder Consola")
    (else
      (return ""))))