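; Breakable oxygen tank that loses oxygen over time, faster at higher damage grades, and shows the percentage on digital terminals.
; A GameMode-bound event toggles breakage, revealing leak meshes according to the damage grade.
; Interacting with leaks while holding tape hides them individually; unless all are sealed within a three-second window, the grade's leaks reappear.
; Tick drives the drain through Delay-based timing; running out only prints a death placeholder.
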(event Custom|Romper/Arreglar
  ;[1 0.5521 0.5521] Romper/Arreglar Tanque de Oxigeno
  (if (Variables|Test|GetRoto?)
    (Variables|Test|SetRoto? false)
    (Variables|Prueba|SetGrado 0)
    (Rendering|SetVisibility (Components|GetChildrenComponents (Variables|Default|GetRoturasScene) false) (Variables|Test|GetRoto?) false)
    (else
      (Variables|Test|SetRoto? true)
      (|GradosRoturas)))
  (if (Variables|Test|GetRoto?)
    (Development|PrintString "Tanque Oxigeno Roto" true true "(R=1.000000,G=0.000000,B=0.000000,A=1.000000)")
    (else
      (Development|PrintString "Tanque Oxigeno Arreglado" true true "(R=0.314782,G=1.000000,B=0.000000,A=1.000000)"))))

(event Custom|AumentarGrado
  ;[1 1 1] Grado Daños
  (if (< (Variables|Prueba|GetGrado) 4)
    (bind _output_get (Variables|Prueba|SetGrado (+ (Variables|Prueba|GetGrado) 1)))
    (Development|PrintString (Utilities|String|Append "Grado Daño Oxigeno " (Utilities|String|ToString(Integer) _output_get)))))

(event Custom|DisminuirGrado
  ;[1 1 1] Grado Daños
  (if (> (Variables|Prueba|GetGrado) 0)
    (bind _output_get (Variables|Prueba|SetGrado (- (Variables|Prueba|GetGrado) 1)))
    (Development|PrintString (Utilities|String|Append "Grado Daño Oxigeno " (Utilities|String|ToString(Integer) _output_get)))))

(event EventObjectInteractions
  (params (SceneComponentTarget :type Scene%20Component%20Object%20Reference))
  ;[1 1 1] Arreglos
  (bind _returnvalue (|ObjetoAManoCinta?))
  (if _returnvalue
    (if (Components|ComponentHasTag SceneComponentTarget "RoturaT")
      (|ArregloRoturasIndividuales SceneComponentTarget
        (:then
          _)
        (:then2
          _)
        (:then3
          _)
        (:then4
          _)
        (:then5
          _)
        (:then6
          _))
      (if (|CondicionArregloTotal)
        (Variables|Test|SetRoto? false)
        (Variables|Prueba|SetGrado 0)
        ;[1 0.5521 0.5521] Romper/Arreglar Tanque de Oxigeno
        (if (Variables|Test|GetRoto?)
          (Development|PrintString "Tanque Oxigeno Roto" true true "(R=1.000000,G=0.000000,B=0.000000,A=1.000000)")
          (else
            (Development|PrintString "Tanque Oxigeno Arreglado" true true "(R=0.314782,G=1.000000,B=0.000000,A=1.000000)")))
        (else
          (|QuickTimeEventCheck))))))

(event EventTick
  (params (DeltaSeconds :type Float%20%28single-precision%29))
  (bind _oxigeno (Variables|Prueba|GetOxigeno))
  ;[1 1 1] Perdida Oxigeno
  (if (> _oxigeno 0.0)
    (if (Variables|Test|GetRoto?)
      (|PerdidaOxigeno :!label _label)
      (else
        (goto _label execute2)))
    (elif (== _oxigeno 0.0)
      (Development|PrintText "SIN OXIGENO - REEMPLAZAR POR LLAMADA A MUERTE "))))

(event EventBeginPlay
  (bind _gamemode (Utilities|GetGameMode)
    (:Is%20Valid
      (EventDispatchers|AssignOxygenBreakEvent _gamemode (delegate Custom|Romper/Arreglar)))))

(fn ConstructionScript)