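; Multi-floor ladder object that the player can mount, climb floor by floor and leave.
; BeginPlay maps the child components of PisosConjunto to floor indices, and interacting with one toggles ladder use, move/look control and Flying or Walking mode.
; While active, directional input steps the floor index to move the player up or down.
; Timelines lerp player location, plus camera rotation when mounting and leaving, with a Delay flag blocking input meanwhile.
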(event Custom|UsarEscalera
  (params (PisoActualIndex :type Integer) (PisoActualObject :type Scene%20Component%20Object%20Reference))
  (bind _returnvalue (Game|GetPlayerCharacter 0))
  (bind _charactermovement (Variables|/Script/Engine.Character|GetCharacterMovement _returnvalue))
  ;[0 1 0.5105] Usar Escalera
  (if (not (Variables|Test|GetDelay)) ; True = Inutilizable por "Delay"\nFalse = Utilizable
    (bind _isa (Utilities|FlowControl|FlipFlop)
      (:A
        _)
      (:B
        _))
    (Variables|Test|SetActivo? _isa) ; True = Utilizandose por Jugador\nFalse = No utilizandose
    (Utilities|Habilitar/DeshabilitarMove&Look _isa)
    (if _isa
      ;;[1 1 1] Usar la Escalera
      (Variables|Test|SetPisoActualIndex PisoActualIndex) ; Index del Piso
      (Variables|Default|SetPisoActualComponent PisoActualObject)
      (CallFunction|MovimientoHaciaEscalera (Transformation|GetWorldLocation PisoActualObject))
      (Pawn|Components|CharacterMovement|SetMovementMode _charactermovement "MOVE_Flying" 0) ; Habilita el modo de vuelo, para que el jugador\npueda ir hacia arriba
      (else
        ;;[1 1 1] Salir de Escalera
        (CallFunction|SalirDeEscalera)
        (Pawn|Components|CharacterMovement|SetMovementMode _charactermovement "MOVE_Walking" 0)))))

(event Custom|MovimientoHaciaEscalera
  (params (LocalizacionPisoActual :type Vector))
  ;[1 0.7996 0.2266] Movimiento hacia Escalera (Usar Escalera)
  (CallFunction|ObtLocalizacion-Jugador)
  ;;[0 0.7402 1] Animacion - Timelapse
  (bind (_direction _movimientocuerpo _movimientocamara) (Timeline|Movimiento PlayFromStart)
    (:Update
      (Variables|Test|SetDelay true)
      (Utilities|MovimientoDeJugadorHaciaEscalera (Variables|Posicionamiento|GetPlayerCurrentLocation) (.x LocalizacionPisoActual) (.y LocalizacionPisoActual) _movimientocuerpo)
      (Utilities|RotacionHaciaEscalera (.x LocalizacionPisoActual) (.y LocalizacionPisoActual) _movimientocamara))
    (:Finished
      (Variables|Test|SetDelay false))))

(event Custom|Subir/Bajar%20Pisos
  (params (Input :type Float%20%28double-precision%29))
  ;[1 0.7996 0.2266] Subir/Bajar Pisos
  (Utilities|InputPositivo/Negativo Input
    (:Input1
      (bind _outputindex (Utilities|Aumento/DisminucionIndex (Variables|Test|GetPisoActualIndex) (CallFunction|ObtCantidadDePisos) :!label _label)
        (:Output1
          _)
        (:Output2
          _))
      (CallFunction|ObtLocalizacion-Jugador)
      ;;[0 0.7402 1] Animacion - Timelapse
      (bind _movimientoescalera (Timeline|Subir/Bajar%20Escalera PlayFromStart)
        (:Update
          (Variables|Test|SetDelay true)
          (Utilities|MovimientoDeJugadorSubir/Bajar (Variables|Posicionamiento|GetPlayerCurrentLocation) (.Return%20Value%20X (CallFunction|ObtLocalizacion-Piso _outputindex)) (.Return%20Value%20Y (CallFunction|ObtLocalizacion-Piso _outputindex)) (.Return%20Value%20Z (CallFunction|ObtLocalizacion-Piso _outputindex)) _movimientoescalera))
        (:Finished
          (Variables|Test|SetDelay false))))
    (:Input2
      (goto _label Input2))))

(event Custom|Salir%20de%20escalera
  (bind _pisoactualindex (Variables|Test|GetPisoActualIndex))
  (bind (_return_value_x _return_value_y _return_value_z) (CallFunction|ObtLocalizacion-Piso _pisoactualindex))
  ;[1 0.7996 0.2266] Subir/Bajar Pisos
  (CallFunction|ObtLocalizacion-Jugador)
  ;;[0 0.7402 1] Animacion - Timelapse
  (bind (_direction _movimientoescalera _rotacionescalera) (Timeline|Timeline PlayFromStart)
    (:Update
      (Variables|Test|SetDelay true)
      (Utilities|MovimientoDeJugadorSalir (Variables|Posicionamiento|GetPlayerCurrentLocation) _return_value_x _return_value_y _return_value_z _movimientoescalera)
      (Utilities|RotacionSalidaDeEscalera _return_value_x _return_value_y _rotacionescalera))
    (:Finished
      (Variables|Test|SetDelay false))))

(event EventObjectInteractions
  (params (SceneComponentTarget :type Scene%20Component%20Object%20Reference))
  ;[0.9471 0.4638 1] Interaccion con Objeto - Uso de Escalera
  (bind (_pisovalido_ _pisoindex _pisovalido) (Utilities|VerificacionDePisoValido SceneComponentTarget)
    (:LoopBody
      (if _pisovalido_ ; Si el piso existe,  usa la escalera
        (CallFunction|UsarEscalera _pisoindex _pisovalido)))))

(event EventBeginPlay
  (Utilities|OrganizacionDePisos) ; Obtiene cada piso en "PisosConjunto", determinando\nun Index (valor) a cada piso al iniciar el juego.
)

(event EventObjectW/Input
  (params (InputValor :type Float%20%28double-precision%29))
  ;[0.9471 0.4638 1] Evento Con Input - Subida/Bajada de Pisos
  (if (Variables|Test|GetActivo?)
    (if (not (Variables|Test|GetDelay))
      (CallFunction|Subir/BajarPisos InputValor))))

(fn ConstructionScript)

(fn ObtLocalizacion-Jugador
  (Variables|Posicionamiento|SetPlayerCurrentLocation (Transformation|GetActorLocation (Game|GetPlayerCharacter 0)))
  (return))

(fn ObtLocalizacion-Piso
  (params (IndexPiso :type Integer%20%28by%20ref%29))
  (bind _cantidaddepisos (Variables|Test|GetCantidadDePisos))
  (bind _value (Utilities|Map|Find _cantidaddepisos IndexPiso))
  (bind _returnvalue (Transformation|GetWorldLocation _value))
  (return (.x _returnvalue) (.y _returnvalue) (.z _returnvalue)))

(fn ObtCantidadDePisos
  (return (- (Utilities|Map|Length (Variables|Test|GetCantidadDePisos)) 1)))