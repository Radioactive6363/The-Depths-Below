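; Spotlight actor that flickers and switches off or on in response to a random-light event from the game mode.
; On BeginPlay it applies a dynamic flickering material as the spotlight's light function and binds RandomLightEvent to the game mode's dispatcher.
; That event enables flicker at random speed and sets a random-delay, one-shot timer for TurnLights.
; TurnLights alternates the material's on/off parameter through a FlipFlop, starting with off.
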(event Custom|RandomLightEvent
  (params (MaxTime :type Float%20%28double-precision%29))
  (switch int (Math|Random|RandomInteger 0)
    (:0
      (Rendering|Material|SetScalarParameterValue (Variables|Default|GetCausticLights) "LerpToFlickering" 1.0 :!class /Script/Engine.MaterialInstanceDynamic) ; 1 = Titilieo\n0 = LuzNormal
      (Rendering|Material|SetScalarParameterValue (Variables|Default|GetCausticLights) "FlickeringSpeed" (Math|Random|RandomFloatinRange 1.0 15.0) :!class /Script/Engine.MaterialInstanceDynamic) ; 1 >= Velocidad\n0 = Sin Movimiento
      (Utilities|Time|SetTimerbyFunctionName 0 "TurnLights" (Math|Random|RandomFloatinRange 5.0 15.0)))))

(event Custom|TurnLights
  (Utilities|FlowControl|FlipFlop
    (:A
      (Rendering|Material|SetScalarParameterValue (Variables|Default|GetCausticLights) "LightsOn/Off" 0.0 :!class /Script/Engine.MaterialInstanceDynamic) ; 1 = LuzPrendida\n0 = LuzApagada
    )
    (:B
      (Rendering|Material|SetScalarParameterValue (Variables|Default|GetCausticLights) "LightsOn/Off" 1.0 :!class /Script/Engine.MaterialInstanceDynamic) ; 1 = LuzPrendida\n0 = LuzApagada
    )))

(event EventBeginPlay
  (Utilities|FlowControl|Sequence
    (:then_0
      (bind _returnvalue (Rendering|Material|CreateDynamicMaterialInstance "/Game/Materials/MI_LightFlickering.MI_LightFlickering" "None" "None" :!class /Script/Engine.KismetMaterialLibrary))
      (bind _output_get (Variables|Default|SetCausticLights _returnvalue))
      (Rendering|Components|Light|SetLightFunctionMaterial (Variables|Default|GetSpotLight) _output_get))
    (:then_1
      (bind _gamemode (Utilities|GetGameMode)
        (:Is%20Valid
          (EventDispatchers|BindEventtoRandomDispatcher _gamemode (delegate Custom|RandomLightEvent)))))))

(fn ConstructionScript)