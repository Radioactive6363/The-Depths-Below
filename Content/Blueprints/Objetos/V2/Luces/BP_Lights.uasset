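; Light fixture actor whose mesh and rect light can flicker, switch off and reset on cues from the game mode.
; One dynamic MI_LightFlickering instance drives both the mesh material and light function through scalar parameters.
; Game mode events trigger flickering with audio at random speed, or restore steady light.
; The event selector is fixed to Evento2, leaving Evento1's timed blackout with sparks and random sound unused.
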(event Custom|RandomLightEvent
  (params (MaxTime :type Float%20%28double-precision%29))
  (switch int 1
    (:0
      (|Evento1 MaxTime))
    (:1
      (|Evento2))))

(event Custom|DesactivarTitileo
  ;[1 1 1] Desactivado Titileo - Luces
  (Rendering|Material|SetScalarParameterValue (Variables|Default|GetLightsFlickeringMats) "LerpToFlickering" 0.0 :!class /Script/Engine.MaterialInstanceDynamic) ; 1 = Titilieo\n0 = LuzNormal
)

(event Custom|ApagadoLuces
  (bind _audio (Variables|Default|GetAudio))
  ;[1 1 1] Apagado/Encendido - Luces
  (Audio|Components|Audio|Stop _audio)
  (Audio|PlaySoundatLocation (.OutItem (Utilities|Array|Random (Variables|Default|GetArraySounds))) (Transformation|GetWorldLocation _audio) "0, 0, 0" 1.0 1.0 0.0 "/Game/Audio/Attenuation/LightFlickeringAttenuation.LightFlickeringAttenuation" 0 0 0)
  (Rendering|Material|SetScalarParameterValue (Variables|Default|GetLightsFlickeringMats) "LightsOn/Off" 0.0 :!class /Script/Engine.MaterialInstanceDynamic) ; 1 = LuzPrendida\n0 = LuzApagada
  (Components|Activation|Activate (Variables|Default|GetSparks) false))

(event Custom|ActivarTitileo
  ;[1 1 1] Activado Titileo - Luces
  (Rendering|Material|SetScalarParameterValue (Variables|Default|GetLightsFlickeringMats) "LerpToFlickering" 1.0 :!class /Script/Engine.MaterialInstanceDynamic) ; 1 = Titilieo\n0 = LuzNormal
  (Audio|Components|Audio|Play (Variables|Default|GetAudio) 0.0))

(event Custom|VelocidadTitileo
  ;[1 1 1] Velocidad Titileo - Luces
  (Rendering|Material|SetScalarParameterValue (Variables|Default|GetLightsFlickeringMats) "FlickeringSpeed" (Math|Random|RandomFloatinRange 1.0 3.0) :!class /Script/Engine.MaterialInstanceDynamic) ; 1 >= Velocidad\n0 = Sin Movimiento
)

(event Custom|ReseteoLuces
  ;[1 1 1] Reseteo
  (CallFunction|EncendidoLuces)
  (CallFunction|DesactivarTitileo))

(event Custom|EncendidoLuces
  ;[1 1 1] EncendidoLuces
  (Rendering|Material|SetScalarParameterValue (Variables|Default|GetLightsFlickeringMats) "LightsOn/Off" 1.0 :!class /Script/Engine.MaterialInstanceDynamic) ; 1 = LuzPrendida\n0 = LuzApagada
)

(event EventBeginPlay
  (Utilities|FlowControl|Sequence
    (:then_0
      (bind _returnvalue (Rendering|Material|CreateDynamicMaterialInstance "/Game/Materials/MI_LightFlickering.MI_LightFlickering" "None" "None" :!class /Script/Engine.KismetMaterialLibrary))
      (bind _output_get (Variables|Default|SetLightsFlickeringMats _returnvalue))
      (Rendering|Material|SetMaterial (Variables|Default|GetStaticMesh) 0 _output_get)
      (Rendering|Components|Light|SetLightFunctionMaterial (Variables|Default|GetRectLight) _output_get))
    (:then_1
      (bind _gamemode (Utilities|GetGameMode)
        (:Is%20Valid
          (EventDispatchers|BindEventtoFlickeringLightsEvent _gamemode (delegate Custom|RandomLightEvent))
          (EventDispatchers|BindEventtoResetMainLights _gamemode (delegate Custom|ReseteoLuces)))))))

(fn ConstructionScript)