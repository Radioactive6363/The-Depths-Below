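; BP_Lights3 is a light fixture that reacts to game-wide flickering, alarm and reset events bound through the GameMode.
; On BeginPlay it creates a dynamic MI_LightFlickering material, shared by the mesh and the point light's light function, so scalar parameters drive both.
; Flickering runs until a timer switches the light off; the alarm switches it on in red.
; Reset restores white and stops flickering without switching the light back on.
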(event Custom|Alarma
  (bind _light_mat (Variables|Default|GetLight%20Mat))
  (CallFunction|EncendidoLuces)
  (Rendering|Components|Light|SetLightColor (Variables|Default|GetPointLight) "(R=1.000000,G=0.021823,B=0.000000,A=1.000000)" true)
  (Rendering|Material|SetVectorParameterValue _light_mat "LightColor" "(R=1.000000,G=0.000000,B=0.000000,A=1.000000)" :!class /Script/Engine.MaterialInstanceDynamic)
  (Rendering|Material|SetScalarParameterValue _light_mat "AlarmLight" 1.0 :!class /Script/Engine.MaterialInstanceDynamic))

(event Custom|ApagadoLuces
  ;[1 1 1] Apagado Luces
  (Rendering|Material|SetScalarParameterValue (Variables|Default|GetLight%20Mat) "LightsOn/Off" 0.0 :!class /Script/Engine.MaterialInstanceDynamic) ; 1 = LuzPrendida\n0 = LuzApagada
)

(event Custom|ActivarTitileo
  ;[1 1 1] Activado Titileo - Luces
  (Rendering|Material|SetScalarParameterValue (Variables|Default|GetLight%20Mat) "LerpToFlickering" 1.0 :!class /Script/Engine.MaterialInstanceDynamic) ; 1 = Titilieo\n0 = LuzNormal
)

(event Custom|FlickeringLights%20Start
  (params (MaxTime :type Float%20%28double-precision%29))
  (CallFunction|ActivarTitileo)
  (Utilities|Time|SetTimerbyFunctionName 0 "ApagadoLuces" MaxTime))

(event Custom|DesactivarTitileo
  ;[1 1 1] Desactivado Titileo - Luces
  (Rendering|Material|SetScalarParameterValue (Variables|Default|GetLight%20Mat) "LerpToFlickering" 0.0 :!class /Script/Engine.MaterialInstanceDynamic) ; 1 = Titilieo\n0 = LuzNormal
)

(event Custom|EncendidoLuces
  ;[1 1 1] Encendido Luces
  (Rendering|Material|SetScalarParameterValue (Variables|Default|GetLight%20Mat) "LightsOn/Off" 1.0 :!class /Script/Engine.MaterialInstanceDynamic) ; 1 = LuzPrendida\n0 = LuzApagada
)

(event Custom|Reset
  (bind _light_mat (Variables|Default|GetLight%20Mat))
  (Rendering|Components|Light|SetLightColor (Variables|Default|GetPointLight) "(R=1.000000,G=1.000000,B=1.000000,A=1.000000)" true)
  (Rendering|Material|SetVectorParameterValue _light_mat "LightColor" "(R=1.000000,G=1.000000,B=1.000000,A=1.000000)" :!class /Script/Engine.MaterialInstanceDynamic)
  (Rendering|Material|SetScalarParameterValue _light_mat "AlarmLight" 0.0 :!class /Script/Engine.MaterialInstanceDynamic)
  (CallFunction|DesactivarTitileo))

(event EventBeginPlay
  (Utilities|FlowControl|Sequence
    (:then_0
      (bind _returnvalue (Rendering|Material|CreateDynamicMaterialInstance "/Game/Materials/MI_LightFlickering.MI_LightFlickering" "None" "None" :!class /Script/Engine.KismetMaterialLibrary))
      (bind _output_get (Variables|Default|SetLight%20Mat _returnvalue))
      (Rendering|Material|SetMaterial (Variables|Default|GetStaticMesh) 0 _output_get)
      (Rendering|Components|Light|SetLightFunctionMaterial (Variables|Default|GetPointLight) _output_get))
    (:then_1
      (bind _gamemode (Utilities|GetGameMode)
        (:Is%20Valid
          (EventDispatchers|BindEventtoFlickeringLightsEvent _gamemode (delegate Custom|FlickeringLights%20Start))
          (EventDispatchers|BindEventtoAlarmEvent _gamemode (delegate Custom|Alarma))
          (EventDispatchers|BindEventtoResetMainLights _gamemode (delegate Custom|Reset)))))))

(fn ConstructionScript)