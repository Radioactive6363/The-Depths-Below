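; BP_Coleccionable is a collectible object that tumbles at random until it is attached to a claw (garra) and later handed to the hatch.
; From a random start rotation, a self-restarting Timeline lerps Objeto toward new random rotations.
; Attaching stops the Timeline and snaps it to the claw's socket, keeping world rotation.
; Teleporting sends its reference, bounds and rotation to BP_Escotilla, then detaches it; a separate event enables physics.
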(event Custom|ObjectRandomMovement
  (bind _returnvalue (Math|Random|RandomFloatinRange 0.0 3.6e+02))
  ;[1 1 1] Animacion de Rotacion
  (Variables|Default|SetObjectActualRotation (Variables|/Script/Engine.SceneComponent|GetRelativeRotation (Variables|Default|GetObjeto)))
  (Variables|Default|SetObjectTargetRotation (Math|Rotator|MakeRotator _returnvalue _returnvalue _returnvalue))
  (bind _rotationalpha (Timeline|Timeline PlayFromStart)
    (:Update
      (Transformation|SetRelativeRotation (Variables|Default|GetObjeto) (Math|Rotator|Lerp(Rotator) (Variables|Default|GetObjectActualRotation) (Variables|Default|GetObjectTargetRotation) _rotationalpha true) false false))
    (:Finished
      (CallFunction|ObjectRandomMovement))))

(event EventBeginPlay
  (bind _returnvalue (Math|Random|RandomFloatinRange 0.0 3.6e+02))
  ;[1 1 1] Rotacion Inicial Aleatoria.
  (Transformation|SetRelativeRotation (Variables|Default|GetObjeto) (Math|Rotator|MakeRotator _returnvalue _returnvalue _returnvalue) false false)
  (CallFunction|ObjectRandomMovement))

(event EventTeleporttoHatch
  (bind _objeto (Variables|Default|GetObjeto))
  (bind _returnvalue (Actor|GetActorOfClass "/Game/Blueprints/Objetos/V2/BP_Escotilla.BP_Escotilla_C"))
  (Class|BPIHatch|SendColeccionable(Message) _returnvalue self (.BoxExtent (Collision|GetComponentBounds _objeto)) (Variables|/Script/Engine.SceneComponent|GetRelativeRotation _objeto))
  (Transformation|DetachFromActor "KeepWorld" "KeepWorld" "KeepWorld"))

(event EventActivatePhysics
  (Physics|SetSimulatePhysics (Variables|Default|GetObjeto) true))

(event EventAttachtoGarra
  (params (GarraInput :type Skeletal%20Mesh%20Component%20Object%20Reference))
  (Audio|Components|Audio|Stop (Variables|Default|GetTimeline))
  (Transformation|AttachComponentToComponent GarraInput "Base3_001" "SnapToTarget" "KeepWorld" "KeepWorld" false))

(fn ConstructionScript)