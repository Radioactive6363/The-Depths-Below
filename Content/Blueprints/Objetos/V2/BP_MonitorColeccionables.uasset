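; Interactive collectibles monitor object whose screen is a widget component the player can interact with.
; Interacting triggers a camera change to the monitor's camera, stores the result as the active state, and passes it to the screen's UI widget.
; The hover check offers a "Manage Objects" prompt only when the widget component is hit and the monitor is not already active.
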(event Custom|Cambio%20de%20Camara
  ;[0 0.3354 0.3802] Cambio de Camara
  (bind _isa (Utilities|CameraChange (Variables|Default|GetCamera)))
  (Variables|Default|SetActivo? _isa)
  (Class|BPIInteractions|ObjectActivate(Message) (UserInterface|GetWidget (Variables|Default|GetMonitorColeccionablesUI)) (Variables|Default|GetActivo?)))

(event EventObjectInteractions
  (params (SceneComponentTarget :type Scene%20Component%20Object%20Reference))
  (CallFunction|CambioDeCamara))

(fn ConstructionScript)

(fn IsHoveringActor
  (params (Hit :type Hit%20Result%20Structure) (Player :type Actor%20Object%20Reference))
  (if (and (== (Variables|Default|GetMonitorColeccionablesUI) (.HitComponent (Collision|BreakHitResult Hit))) (not (Variables|Default|GetActivo?)))
    (return "Manage Objects")
    (else
      (return ""))))