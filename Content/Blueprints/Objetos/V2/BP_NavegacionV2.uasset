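; Interactive navigation lever station that lets the player step through three speed settings.
; Interacting with the lever trigger, while usable, flip-flops the view between station camera and player, toggling move and look input.
; While active, navigation input steps a clamped speed index, and a Timeline rotates the lever to that index's angle, disabling player input until finished.
; ObjectActivate sets whether the station is usable, reflecting breaker or motor state.
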(event Custom|CambioDeCamara
  ;[0 0.3354 0.3802] Cambio de Camara
  (bind _isa (Utilities|FlowControl|FlipFlop)
    (:A
      ;;[1 0.4792 0.4792] Camara Navegacion
      (Utilities|Des/HabilitarMove&Look _isa)
      (Game|Player|SetViewTargetwithBlend (Game|GetPlayerController 0) (Components|GetOwner (Variables|Default|GetCamera)) 0.5 "VTBlend_EaseInOut" 1e+01 false))
    (:B
      ;;[1 0.5 0.5] Camara Jugador
      (Utilities|Des/HabilitarMove&Look _isa)
      (Game|Player|SetViewTargetwithBlend (Game|GetPlayerController 0) (Game|Player|GetPlayerPawn 0) 0.5 "VTBlend_EaseInOut" 1e+01 false)))
  (Variables|Test|SetActivo? _isa))

(event Custom|CambioVelocidad
  (params (InputValor :type Float%20%28double-precision%29))
  ;[0.3802 0.1951 0.04189] Cambio de Velocidad
  (if (Variables|Test|GetActivo?) ; True = Player en Navegacion\nFalse = Player NO esta en Navegacion
    (Utilities|FlowControl|Sequence
      (:then_0
        (bind _velocidadesindex (Utilities|Aumento/DisminucionIndex InputValor :!label _label)
          (:AumentoVelocidad
            (bind _palancafloat (Timeline|Timeline PlayFromStart)
              (:Update
                (Input|DisableInput (Game|GetPlayerCharacter 0) (Game|GetPlayerController 0))
                (Transformation|SetRelativeRotation (Variables|Default|GetPalanca) (Math|Rotator|MakeRotator 0.0 (.y (Math|Vector|Lerp(Vector) (Math|Vector|MakeVector 0.0 (Variables|Default|GetAnguloPalancaActual) 0.0) (Math|Vector|MakeVector 0.0 (Utilities|Array|Get(acopy) (Variables|Test|GetAngulosPalanca) _velocidadesindex) 0.0) _palancafloat)) 0.0) false false))
              (:Finished
                (Variables|Default|SetAnguloPalancaActual (Utilities|Array|Get(acopy) (Variables|Test|GetAngulosPalanca) (Variables|Test|GetVelocidadesIndex))) ; Actualizacion del Angulo de la Palanca
                (Input|EnableInput (Game|GetPlayerCharacter 0) (Game|GetPlayerController 0)))))
          (:DisminucionVelocidad
            (Timeline|Timeline PlayFromStart))))
      (:then_1
        (goto _label Disminuir)))))

(event Custom|InutilizacionNavegacion
  (params (Utilizable? :type Boolean))
  ;[1 0 0] Inutilizacion Navegacion (Rotura/Motor Apagado)
  (Variables|Test|SetUtilizable? Utilizable?))

(event Custom|ResetNavegation
  (bind _angulospalanca (Variables|Test|GetAngulosPalanca))
  (bind _velocidadesindex (Variables|Test|GetVelocidadesIndex))
  (bind _output (Utilities|Array|Get(acopy) _angulospalanca _velocidadesindex))
  ;[1 1 1] Reseteo de Valores Iniciales - Movimiento de Palanca (en caso de cambio del Valor del Index)
  ; Unicamente para Inicio y Testeo
  (Transformation|SetRelativeRotation (Variables|Default|GetPalanca) (Math|Rotator|MakeRotator 0.0 _output 0.0) false false)
  (Variables|Default|SetAnguloPalancaActual _output))

(event EventNavegationInput
  (params (InputValor :type Float%20%28double-precision%29))
  ;[1 0.3471 0.9571] Evento Con Input - Cambio de Velocidad
  (CallFunction|CambioVelocidad InputValor))

(event EventObjectInteractions
  (params (ComponentTarget :type Object%20Object%20Reference))
  ;[0.9471 0.4638 1] Interaccion con Objeto - Cambio de Camara
  (if (== ComponentTarget (Variables|Default|GetPalancaTrigger))
    (if (Variables|Test|GetUtilizable?) ; True = Llave Termica Encendida/Motor NO Roto\nFalse =  Llave Termica Apagada/Motor Roto
      (CallFunction|CambioDeCamara))))

(event EventBeginPlay
  (CallFunction|ResetNavegation))

(event EventObjectActivate
  (params (Activate? :type Boolean))
  ;[1 0.3471 0.9571] Accion de Objeto - Inutilizacion Navegacion
  (CallFunction|InutilizacionNavegacion Activate?))

(fn ConstructionScript)