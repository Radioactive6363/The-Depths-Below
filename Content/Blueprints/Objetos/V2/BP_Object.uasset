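; BP_Object is an interactable world object that toggles between a grabbed state and its default physical state.
; Its ObjectInteractions event calls AgarradoDeObjeto, where a FlipFlop alternates on each call between disabling and restoring physics simulation and collision on the mesh and box collider.
; The restored box collider is query-only, while the mesh gets query and physics.
; The file contains no attachment or movement logic, only this toggle with debug prints.
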(event Custom|AgarradoDeObjeto
  (bind _isa (Utilities|FlowControl|FlipFlop)
    (:A
      (Variables|Default|SetTipoDeFisicasMesh "NoCollision") ; Desactivar Colisiones Mesh
      (Variables|Default|SetTipoDeFisicasBoxCollider "NoCollision") ; Desactivar Colisiones BoxCollider
      (Development|PrintString "Desactivo Physics" true true "(R=0.000000,G=0.070262,B=1.000000,A=1.000000)"))
    (:B
      (Variables|Default|SetTipoDeFisicasMesh "QueryAndPhysics") ; Fisicas Predeterminadas Mesh (No cambiar)
      (Variables|Default|SetTipoDeFisicasBoxCollider "QueryOnly") ; Fisicas Predeterminadas BoxCollider (No cambiar)
      (Development|PrintString "Activo Physics" true true "(R=1.000000,G=0.000000,B=0.078311,A=1.000000)")))
  (Physics|SetSimulatePhysics (Variables|Default|GetObjeto) (not _isa))
  (Collision|SetCollisionEnabled (Variables|Default|GetObjeto) (Variables|Default|GetTipoDeFisicasMesh))
  (Collision|SetCollisionEnabled (Variables|Default|GetBoxCollider) (Variables|Default|GetTipoDeFisicasBoxCollider)))

(event EventObjectInteractions
  (params (SceneComponentTarget :type Scene%20Component%20Object%20Reference))
  (CallFunction|AgarradoDeObjeto))

(fn ConstructionScript)