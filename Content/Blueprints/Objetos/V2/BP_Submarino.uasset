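; BP_Submarino is a submarine actor that sets off random water flow effects.
; On BeginPlay it binds RandomFlowEvent to the game mode's WaterFlowEvent dispatcher.
; Each event has roughly a 50% chance to activate one randomly chosen WaterFlow component, without resetting it.
; RandomInteger(4) only yields 0 to 3, so the branch for WaterFlow5 never runs.
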(event Custom|RandomFlowEvent
  (if (> (Math|Random|RandomFloatinRange 0.0 1e+02) 5e+01)
    (switch int (Math|Random|RandomInteger 4)
      (:0
        (Components|Activation|Activate (Variables|Default|GetWaterFlow1) false))
      (:1
        (Components|Activation|Activate (Variables|Default|GetWaterFlow2) false))
      (:2
        (Components|Activation|Activate (Variables|Default|GetWaterFlow3) false))
      (:3
        (Components|Activation|Activate (Variables|Default|GetWaterFlow4) false))
      (:4
        (Components|Activation|Activate (Variables|Default|GetWaterFlow5) false)))))

(event EventBeginPlay
  (bind _gamemode (Utilities|GetGameMode)
    (:Is%20Valid
      (EventDispatchers|BindEventtoWaterFlowEvent _gamemode (delegate Custom|RandomFlowEvent)))))

(fn ConstructionScript)