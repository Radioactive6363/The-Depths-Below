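; Black box collectible that tumbles through looping random rotation lerps until the claw (garra) grabs it.
; On first reaching zero height, it plays the sonar UI sound and increments the camera's point-of-interest count.
; Until collected, Tick caps its height, destroying it after enough capped frames.
; Hatch delivery or destruction decrements that count and removes the first entry from the map movement actor's object coordinates.
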(event Custom|ObjectRandomMovement
  (bind _returnvalue (Math|Random|RandomFloatinRange 0.0 3.6e+02))
  ;[1 1 1] Animacion de Rotacion
  (Variables|Default|SetObjectActualRotation (Variables|/Script/Engine.SceneComponent|GetRelativeRotation (Variables|Default|GetObjeto)))
  (Variables|Default|SetObjectTargetRotation (Math|Rotator|MakeRotator _returnvalue _returnvalue _returnvalue))
  (bind _rotationalpha (Timeline|Timeline PlayFromStart)
    (:Update
      (Transformation|SetRelativeRotation (Variables|Default|GetObjeto) (Math|Rotator|Lerp(Rotator) (Variables|Default|GetObjectActualRotation) (Variables|Default|GetObjectTargetRotation) _rotationalpha true) false false))
    (:Finished
      (CallFunction|ObjectRandomMovement))))

(event EventBeginPlay
  (bind _returnvalue (Math|Random|RandomFloatinRange 0.0 3.6e+02))
  ;[1 1 1] Rotacion Inicial Aleatoria.
  (Transformation|SetRelativeRotation (Variables|Default|GetObjeto) (Math|Rotator|MakeRotator _returnvalue _returnvalue _returnvalue) false false)
  (CallFunction|ObjectRandomMovement))

(event EventTeleporttoHatch
  (bind _objeto (Variables|Default|GetObjeto))
  (Variables|Default|SetRegocido true)
  (bind _returnvalue (Actor|GetActorOfClass "/Game/Blueprints/Objetos/V2/BP_Escotilla.BP_Escotilla_C"))
  (Class|BPIHatch|SendColeccionable(Message) _returnvalue self (.BoxExtent (Collision|GetComponentBounds _objeto)) (Variables|/Script/Engine.SceneComponent|GetRelativeRotation _objeto))
  (Transformation|DetachFromActor "KeepWorld" "KeepWorld" "KeepWorld")
  (bind _returnvalue_2 (Actor|GetActorOfClass "/Game/Blueprints/Objetos/V2/BP_MovimientoMapa.BP_MovimientoMapa_C"))
  (bind _keys (Utilities|Map|Keys (Variables|/Game/Blueprints/Objetos/V2/BP_MovimientoMapa.BP_MovimientoMapa_C|GetCoordenadasObjetos _returnvalue_2)))
  (for (_array_element _array_index) _keys
    (if (== _array_index 0)
      (bind _output_get (Variables|/Game/Blueprints/Objetos/V2/BP_MovimientoMapa.BP_MovimientoMapa_C|SetCoordenadasObjetos _returnvalue_2 (Variables|/Game/Blueprints/Objetos/V2/BP_MovimientoMapa.BP_MovimientoMapa_C|GetCoordenadasObjetos _returnvalue_2)))
      (Utilities|Map|Remove _output_get _array_element)))
  (bind _returnvalue_3 (Actor|GetActorOfClass "/Game/Blueprints/Objetos/V2/BP_Camara.BP_Camara_C"))
  (bind _asbp_punto_interes (Utilities|Casting|CastToBP_PuntoInteres (UserInterface|GetWidget (Variables|/Game/Blueprints/Objetos/V2/BP_Camara.BP_Camara_C|GetCoordColecc _returnvalue_3))))
  (Variables|/Game/Blueprints/UI/Objetos/V2/BP_PuntoInteres.BP_PuntoInteres_C|Setcantidad _asbp_punto_interes (- (Variables|/Game/Blueprints/UI/Objetos/V2/BP_PuntoInteres.BP_PuntoInteres_C|Getcantidad _asbp_punto_interes) 1)))

(event EventActivatePhysics
  (Physics|SetSimulatePhysics (Variables|Default|GetObjeto) true))

(event EventAttachtoGarra
  (params (GarraInput :type Skeletal%20Mesh%20Component%20Object%20Reference))
  (Audio|Components|Audio|Stop (Variables|Default|GetTimeline))
  (Transformation|AttachComponentToComponent GarraInput "Base3_001" "SnapToTarget" "KeepWorld" "KeepWorld" false))

(event EventTick
  (params (DeltaSeconds :type Float%20%28single-precision%29))
  (bind _returnvalue (Transformation|GetActorLocation))
  (if (not (Variables|Default|GetRegocido))
    (if (== (Math|Float|Truncate (.z _returnvalue)) 0)
      (if (Variables|Default|GetInicial)
        (Variables|Default|SetInicial false)
        (Utilities|FlowControl|Delay 0.2)
        (Variables|Default|SetposCaja 0.0)
        (bind _returnvalue_2 (Actor|GetActorOfClass "/Game/Blueprints/Objetos/V2/BP_SonarV2.BP_SonarV2_C"))
        (bind _asbp_sonar_uiv2 (Utilities|Casting|CastToBP_SonarUIV2 (UserInterface|GetWidget (Variables|/Game/Blueprints/Objetos/V2/BP_SonarV2.BP_SonarV2_C|GetSonarUI _returnvalue_2))))
        (Default|SonidoColecc _asbp_sonar_uiv2)
        (bind _returnvalue_3 (Actor|GetActorOfClass "/Game/Blueprints/Objetos/V2/BP_Camara.BP_Camara_C"))
        (bind _asbp_punto_interes (Utilities|Casting|CastToBP_PuntoInteres (UserInterface|GetWidget (Variables|/Game/Blueprints/Objetos/V2/BP_Camara.BP_Camara_C|GetCoordColecc _returnvalue_3))))
        (Variables|/Game/Blueprints/UI/Objetos/V2/BP_PuntoInteres.BP_PuntoInteres_C|Setcantidad _asbp_punto_interes (+ (Variables|/Game/Blueprints/UI/Objetos/V2/BP_PuntoInteres.BP_PuntoInteres_C|Getcantidad _asbp_punto_interes) 1)))
      (elif (> (Math|Float|Truncate (.z _returnvalue)) 126)
        (if (< (Variables|Default|GetposCaja) 7.5e+02)
          (Transformation|SetActorLocation (Math|Vector|MakeVector (.x _returnvalue) (.y _returnvalue) 126.0) false false)
          (Variables|Default|SetposCaja (+ (Variables|Default|GetposCaja) 1.0))
          (else
            (Variables|Default|SetposCaja 0.0)
            (bind _returnvalue_4 (Actor|GetActorOfClass "/Game/Blueprints/Objetos/V2/BP_MovimientoMapa.BP_MovimientoMapa_C"))
            (bind _keys (Utilities|Map|Keys (Variables|/Game/Blueprints/Objetos/V2/BP_MovimientoMapa.BP_MovimientoMapa_C|GetCoordenadasObjetos _returnvalue_4)))
            (for (_array_element _array_index) _keys
              (if (== _array_index 0)
                (bind _output_get (Variables|/Game/Blueprints/Objetos/V2/BP_MovimientoMapa.BP_MovimientoMapa_C|SetCoordenadasObjetos _returnvalue_4 (Variables|/Game/Blueprints/Objetos/V2/BP_MovimientoMapa.BP_MovimientoMapa_C|GetCoordenadasObjetos _returnvalue_4)))
                (Utilities|Map|Remove _output_get _array_element)))
            (Actor|DestroyActor)
            (bind _returnvalue_5 (Actor|GetActorOfClass "/Game/Blueprints/Objetos/V2/BP_Camara.BP_Camara_C"))
            (bind _asbp_punto_interes_2 (Utilities|Casting|CastToBP_PuntoInteres (UserInterface|GetWidget (Variables|/Game/Blueprints/Objetos/V2/BP_Camara.BP_Camara_C|GetCoordColecc _returnvalue_5))))
            (Variables|/Game/Blueprints/UI/Objetos/V2/BP_PuntoInteres.BP_PuntoInteres_C|Setcantidad _asbp_punto_interes_2 (- (Variables|/Game/Blueprints/UI/Objetos/V2/BP_PuntoInteres.BP_PuntoInteres_C|Getcantidad _asbp_punto_interes_2) 1))))))))

(fn ConstructionScript)