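; Hatch actor that presents a received collectible through an animated opening, with sound and a travelling light.
; SendColeccionable places the object inside, then chained timelines raise the hatch and slide object and light horizontally to a final point, where the object's physics activates.
; When the collectible leaves the overlap box, its reference is cleared and the same timelines reverse, returning the light and then closing the hatch.
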(event OnComponentEndOverlap(BoxOverlap)
  (params (OverlappedComponent :type Primitive%20Component%20Object%20Reference) (OtherActor :type Actor%20Object%20Reference) (OtherComp :type Primitive%20Component%20Object%20Reference) (OtherBodyIndex :type Integer))
  (bind _posactualluz (Variables|Default|GetPosActualLuz))
  (bind _posactualobjeto (Variables|Default|GetPosActualObjeto))
  (bind _posicionfinal (Variables|Default|GetPosicionFinal))
  (bind _posicionfinal_2 (Variables|Default|GetPosicionFinal))
  (bind _returnvalue (Transformation|GetWorldLocation _posicionfinal_2))
  (bind _returnvalue_2 (Transformation|GetWorldLocation _posicionfinal))
  ;[1 1 1] Entrada de Objeto - Animacion
  ;;[1 0 0] Revertir Animacion cuando Coleccionable se Agarra
  (if (== OtherActor (Variables|Default|GetObjetoColeccionable))
    (Variables|Default|SetObjetoColeccionable 0)
    (bind _entradaobjecto (Timeline|Salida%20Objeto ReverseFromEnd)
      (:Update
        ;;[1 0 0] Si el objeto no es valido, no se toma en cuenta
        (Utilities|IsValid (Variables|Default|GetObjetoColeccionable)
          (:Is%20Valid
            (Transformation|SetActorLocation (Variables|Default|GetObjetoColeccionable) (Math|Vector|Lerp(Vector) (Math|Vector|MakeVector (.x _posactualobjeto) (.y _posactualobjeto) (.z _posactualobjeto)) (Math|Vector|MakeVector (.x _returnvalue_2) (.y _returnvalue_2) (.z _posactualobjeto)) _entradaobjecto) false false)
            (Transformation|SetWorldLocation (Variables|Default|GetLuzActor) (Math|Vector|Lerp(Vector) (Math|Vector|MakeVector (.x _posactualluz) (.y _posactualluz) (.z _posactualluz)) (Math|Vector|MakeVector (.x _returnvalue) (.y _returnvalue) (.z _posactualluz)) _entradaobjecto) false false))
          (:Is%20Not%20Valid
            ;;[1 0 0] Cerrado de Escotilla
            (Transformation|SetWorldLocation (Variables|Default|GetLuzActor) (Math|Vector|Lerp(Vector) (Math|Vector|MakeVector (.x _posactualluz) (.y _posactualluz) (.z _posactualluz)) (Math|Vector|MakeVector (.x _returnvalue) (.y _returnvalue) (.z _posactualluz)) _entradaobjecto) false false))))
      (:Finished
        (Utilities|IsValid (Variables|Default|GetObjetoColeccionable)
          (:Is%20Valid
            (Class|BPIColeccionableHaciaGarra|ActivatePhysics(Message) (Variables|Default|GetObjetoColeccionable)))
          (:Is%20Not%20Valid
            (CallFunction|EscotillaAnimReverse)))))))

(event Custom|EscotillaAnim
  ;[0.6993 0.6302 1] Escotilla Apertura - Animacion
  (Variables|Default|SetPosActualEscotilla (Variables|/Script/Engine.SceneComponent|GetRelativeLocation (Variables|Default|GetEscotillaMesh)))
  (Audio|PlaySoundatLocation "/Game/Audio/HatchOpen.HatchOpen" (Transformation|GetActorLocation) "0, 0, 0" 1.0 1.0 0.0 "/Game/Audio/Attenuation/AttenuationSettingsHatch.AttenuationSettingsHatch" 0 0 0)
  (bind _hatchmovimientoalpha (Timeline|MovimientoEscotilla PlayFromStart)
    (:Update
      (Transformation|SetRelativeLocation (Variables|Default|GetEscotillaMesh) (Math|Vector|MakeVector (.x (Variables|Default|GetPosActualEscotilla)) (.y (Variables|Default|GetPosActualEscotilla)) (Math|Float|Lerp 0.0 8e+01 _hatchmovimientoalpha)) false false))
    (:Finished
      (Utilities|IsValid (Variables|Default|GetObjetoColeccionable)
        (:Is%20Valid
          (CallFunction|ObjectEntryAnimation))))))

(event Custom|ObjectEntryAnimation
  (bind _posicionfinal (Variables|Default|GetPosicionFinal))
  (bind _objetocoleccionable (Variables|Default|GetObjetoColeccionable))
  (bind _objetocoleccionable_2 (Variables|Default|GetObjetoColeccionable))
  (bind _posicionfinal_2 (Variables|Default|GetPosicionFinal))
  (bind _returnvalue (Transformation|GetWorldLocation _posicionfinal_2))
  (bind _returnvalue_2 (Transformation|GetWorldLocation _posicionfinal))
  ;[1 1 1] Entrada de Objeto - Animacion
  (Variables|Default|SetPosActualObjeto (Transformation|GetActorLocation (Variables|Default|GetObjetoColeccionable)))
  (Variables|Default|SetPosActualLuz (Transformation|GetWorldLocation (Variables|Default|GetLuzActor)))
  (Audio|PlaySoundatLocation "/Game/Audio/ObjectEntry.ObjectEntry" (Transformation|GetActorLocation) "0, 0, 0" 1.0 1.0 0.0 "/Game/Audio/Attenuation/AttenuationSettingsHatch.AttenuationSettingsHatch" 0 0 0)
  (bind _entradaobjecto (Timeline|Salida%20Objeto PlayFromStart)
    (:Update
      ;;[1 0 0] Si el objeto no es valido, no se toma en cuenta
      (Utilities|IsValid _objetocoleccionable
        (:Is%20Valid
          (Transformation|SetActorLocation _objetocoleccionable (Math|Vector|Lerp(Vector) (Math|Vector|MakeVector (.x (Variables|Default|GetPosActualObjeto)) (.y (Variables|Default|GetPosActualObjeto)) (.z (Variables|Default|GetPosActualObjeto))) (Math|Vector|MakeVector (.x _returnvalue_2) (.y _returnvalue_2) (.z (Variables|Default|GetPosActualObjeto))) _entradaobjecto) false false)
          (Transformation|SetWorldLocation (Variables|Default|GetLuzActor) (Math|Vector|Lerp(Vector) (Math|Vector|MakeVector (.x (Variables|Default|GetPosActualLuz)) (.y (Variables|Default|GetPosActualLuz)) (.z (Variables|Default|GetPosActualLuz))) (Math|Vector|MakeVector (.x _returnvalue) (.y _returnvalue) (.z (Variables|Default|GetPosActualLuz))) _entradaobjecto) false false))
        (:Is%20Not%20Valid
          ;;[1 0 0] Cerrado de Escotilla
          (Transformation|SetWorldLocation (Variables|Default|GetLuzActor) (Math|Vector|Lerp(Vector) (Math|Vector|MakeVector (.x (Variables|Default|GetPosActualLuz)) (.y (Variables|Default|GetPosActualLuz)) (.z (Variables|Default|GetPosActualLuz))) (Math|Vector|MakeVector (.x _returnvalue) (.y _returnvalue) (.z (Variables|Default|GetPosActualLuz))) _entradaobjecto) false false))))
    (:Finished
      (Utilities|IsValid _objetocoleccionable_2
        (:Is%20Valid
          (Class|BPIColeccionableHaciaGarra|ActivatePhysics(Message) _objetocoleccionable_2))
        (:Is%20Not%20Valid
          (CallFunction|EscotillaAnimReverse))))))

(event Custom|EscotillaAnimReverse
  (bind _posactualescotilla (Variables|Default|GetPosActualEscotilla))
  ;[0.6993 0.6302 1] Escotilla Apertura - Animacion
  ;;[1 0.1661 0.8408] Escotilla Cerrado - Revertido
  (bind _hatchmovimientoalpha (Timeline|MovimientoEscotilla ReverseFromEnd)
    (:Update
      (Transformation|SetRelativeLocation (Variables|Default|GetEscotillaMesh) (Math|Vector|MakeVector (.x _posactualescotilla) (.y _posactualescotilla) (Math|Float|Lerp 0.0 8e+01 _hatchmovimientoalpha)) false false))
    (:Finished
      (Utilities|IsValid (Variables|Default|GetObjetoColeccionable)
        (:Is%20Valid
          (CallFunction|ObjectEntryAnimation))))))

(event EventSendColeccionable
  (params (ActorReference :type Actor%20Object%20Reference) (Bounds :type Vector :default "0, 0, 0") (Rotation :type Rotator :default "0, 0, 0"))
  (bind _output_get (Variables|Default|SetObjetoColeccionable ActorReference))
  (Transformation|SetActorLocation _output_get (+ (Transformation|GetWorldLocation (Variables|Default|GetPosicionPrincipal)) (Math|Vector|MakeVector 0.0 0.0 (.z Bounds))) false false)
  (Transformation|SetActorRotation (Variables|Default|GetObjetoColeccionable) (Math|Rotator|MakeRotator 0.0 0.0 (.yaw Rotation)))
  (Utilities|Time|SetTimerbyEvent (delegate Custom|EscotillaAnim) 0.1))

(fn ConstructionScript)