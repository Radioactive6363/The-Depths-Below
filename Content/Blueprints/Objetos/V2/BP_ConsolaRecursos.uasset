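; BP_ConsolaRecursos is an interactable resource console that the player enters and exits through the same interaction.
; ObjectInteractions calls Use, whose FlipFlop alternates between console and character modes.
; Entering blends the view to the console camera, switches to Game and UI input, and focuses the InputText of its BP_ConsolaRecursosUI widget.
; Exiting restores the pawn view and game-only input; both character mouse-state functions only cast to BP_PersonajeV2.
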(event Custom|Use
  ;[1 1 1] Accion Entrar y Salir
  (Utilities|FlowControl|FlipFlop
    (:A
      (|CambiarCamaraaConsola)
      (|ModoInputUI)
      (|EstablecerEstadoMouseActivoenPersonaje))
    (:B
      (|CambiarCamaraaPersonaje)
      (|ModoInputJuego)
      (|EstablecerEstadoMouseInactivoenPersonaje))))

(event EventObjectInteractions
  (params (SceneComponentTarget :type Scene%20Component%20Object%20Reference))
  ;[1 1 1] Interaccion
  (CallFunction|Use))

(fn ConstructionScript)