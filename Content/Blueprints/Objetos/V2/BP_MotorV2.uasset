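; Engine actor that switches vertical and horizontal navigation on or off and can break down during play.
; A GameMode event raises a damage grade using the level-name digit, showing breaks and sparks while progressively disabling sonar UI, navigation and the thermal switch (LlaveTermica).
; Interacting with tagged breaks while holding the Soplete repairs them individually, with a three-second E-hold check.
; Full repair resets the grade and restores the sonar UI and thermal switch.
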(event Custom|Romper/Arreglar
  ;[1 0.5521 0.5521] Romper/Arreglar Motor
  (Variables|Test|SetRoto? true)
  (bind _returnvalue (|GradoPorNivel)
    (:then
      (bind _output_get (Variables|Prueba|SetGrado _returnvalue)))
    (:then2
      _))
  (Development|PrintString (Utilities|String|Append "Grado Daño Motor " (Utilities|String|ToString(Integer) _output_get)))
  (|GradosRoturas)
  (if (Variables|Test|GetRoto?)
    (Development|PrintString "Motor Roto" true true "(R=1.000000,G=0.000000,B=0.000000,A=1.000000)")
    (else
      (Development|PrintString "Motor Arreglado" true true "(R=0.314782,G=1.000000,B=0.000000,A=1.000000)"))))

(event Custom|Encendido/Apagado
  (params (Activate? :type Boolean))
  ;[1 0.5521 0.5521] Encendido/Apagado
  (bind _output_get (Variables|Test|SetEncendido? Activate?))
  (Audio|Components|Audio|Play (Variables|Default|GetAudio) 0.0)
  (for _array_element (Variables|Test|GetNavegation)
    (Class|BPIInteractions|ObjectActivate(Message) _array_element _output_get) ; Utilizable?
  ))

(event EventObjectInteractions
  (params (SceneComponentTarget :type Scene%20Component%20Object%20Reference))
  ;[1 1 1] Arreglos
  (if (Variables|Test|GetRoto?)
    (bind (_returnvalue _objeto_a_mano) (|ObjetoAManoSoplete?))
    (if _returnvalue
      (if (Components|ComponentHasTag SceneComponentTarget "RoturaM")
        (Class|BPIInteractions|ObjectActivate(Message) _objeto_a_mano true)
        (|MantenerPresionado3Segundos _objeto_a_mano)
        (|ArregloRoturasIndividuales SceneComponentTarget)
        (if (|CondicionArregloTotal)
          (Variables|Test|SetRoto? false)
          (Variables|Prueba|SetGrado 0)
          (|HabilitarComponentes))))))

(event EventObjectActivate
  (params (Activate? :type Boolean))
  ;[0.9471 0.4638 1] Accion de Objeto - Encendido/Apagado
  (CallFunction|Encendido/Apagado Activate?))

(event EventBeginPlay
  (bind _returnvalue (Actor|GetActorOfClass "/Game/Blueprints/Objetos/V2/BPC_Soplete.BPC_Soplete_C"))
  (Variables|Prueba|SetSopleteRef _returnvalue)
  (Utilities|FlowControl|Sequence
    (:then_0
      ;[0.4683 0.5093 1 1 10] Obtencion de Navegacion
      (bind _returnvalue_2 (Actor|GetActorOfClass "/Game/Blueprints/Objetos/V2/BP_NavegacionVertical.BP_NavegacionVertical_C"))
      (Utilities|Array|Add (Variables|Test|GetNavegation) _returnvalue_2))
    (:then_1
      (bind _returnvalue_3 (Actor|GetActorOfClass "/Game/Blueprints/Objetos/V2/BP_NavegacionHorizontal.BP_NavegacionHorizontal_C"))
      (Utilities|Array|Add (Variables|Test|GetNavegation) _returnvalue_3))
    (:then_2
      (bind _returnvalue_4 (Actor|GetActorOfClass "/Game/Blueprints/Objetos/V2/BP_LlaveTermica.BP_LlaveTermica_C"))
      (bind _output_get (Variables|Test|SetLlave%20Termica%20Reference _returnvalue_4))
      (Utilities|IsValid _output_get
        (:Is%20Not%20Valid
          (Development|PrintString "Falta de Llave Termica en BP_Motor"))))
    (:then_3
      (bind _gamemode (Utilities|GetGameMode)
        (:Is%20Valid
          (EventDispatchers|BindEventtoMotorBreakEvent _gamemode (delegate Custom|Romper/Arreglar)))))))

(fn ConstructionScript)