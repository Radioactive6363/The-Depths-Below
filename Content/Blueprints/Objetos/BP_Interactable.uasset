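; BP_Interactable is an interactable object that toggles the player's view between its camera and the player pawn.
; Interact calls Use, where a FlipFlop alternates between eased view-target blends to the camera's owner and back to the pawn.
; On returning, it also clears EstadoInteract on BP_Personaje and restores walking movement; the file never sets that state or disables movement itself.
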(event Custom|Use
  (bind _returnvalue (Game|GetPlayerCharacter 0))
  (Utilities|FlowControl|FlipFlop
    (:A
      (Game|Player|SetViewTargetwithBlend (Game|GetPlayerController 0) (Components|GetOwner (Variables|Default|GetCamera)) 0.5 "VTBlend_EaseInOut" 1e+01 false))
    (:B
      (Game|Player|SetViewTargetwithBlend (Game|GetPlayerController 0) (Game|Player|GetPlayerPawn 0) 0.5 "VTBlend_EaseInOut" 1e+01 false)
      (bind _asbp_personaje (Utilities|Casting|CastToBP_Personaje _returnvalue))
      (Variables|/Game/Blueprints/Personaje/BP_Personaje.BP_Personaje_C|SetEstadoInteract _asbp_personaje false)
      (Pawn|Components|CharacterMovement|SetMovementMode (Variables|/Script/Engine.Character|GetCharacterMovement _returnvalue) "MOVE_Walking" 0))))

(event EventBeginPlay)

(event Collision|EventActorBeginOverlap
  (params (OtherActor :type Actor%20Object%20Reference)))

(event EventTick
  (params (DeltaSeconds :type Float%20%28single-precision%29)))

(event EventInteract
  (CallFunction|Use))

(fn ConstructionScript)