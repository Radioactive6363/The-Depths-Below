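; BP_TanqueOxigeno is an oxygen tank that randomly breaks and is repaired one breach at a time.
; Tick uses a delayed random roll to set Roto and show three breach components, re-showing them after a delay when CondicionArranqueTimer passes.
; Interact hides the breach matching NombreRotura and clears Roto once all are hidden.
; The visibility test in CondicionArranqueTimer is left unconnected.
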(event Custom|Arreglar
  (bind _nombrerotura (Variables|Default|GetNombreRotura))
  (bind _rotura1 (Variables|Default|GetRotura1))
  (bind _rotura2 (Variables|Default|GetRotura2))
  (bind _rotura3 (Variables|Default|GetRotura3))
  (if (Utilities|Enum|Equal(Enum) _nombrerotura (Utilities|String|ToString(Object) _rotura1))
    (Rendering|SetVisibility _rotura1 false false)
    (if (and (not (Rendering|IsVisible (Variables|Default|GetRotura3))) (Math|Boolean|NORBoolean (Rendering|IsVisible (Variables|Default|GetRotura1)) (Rendering|IsVisible (Variables|Default|GetRotura2)))) :!label _label
      (Variables|Default|Setroto false))
    (elif (Utilities|Enum|Equal(Enum) _nombrerotura (Utilities|String|ToString(Object) _rotura2))
      (Rendering|SetVisibility _rotura2 false false)
      (goto _label)
      (elif (Utilities|Enum|Equal(Enum) _nombrerotura (Utilities|String|ToString(Object) _rotura3))
        (Rendering|SetVisibility _rotura3 false false)
        (goto _label)))))

(event EventBeginPlay)

(event Collision|EventActorBeginOverlap
  (params (OtherActor :type Actor%20Object%20Reference)))

(event EventTick
  (params (DeltaSeconds :type Float%20%28single-precision%29))
  (if (Variables|Default|Getroto)
    (if (|CondicionArranqueTimer)
      (Utilities|FlowControl|Delay 3.0)
      (Rendering|SetVisibility (Variables|Default|GetRotura1) true false))
    (else
      (Utilities|FlowControl|Delay 1.0)
      (switch int (Math|Random|RandomIntegerinRange 0 5)
        (:0
          (Variables|Default|Setroto true)
          (Rendering|SetVisibility (Variables|Default|GetRotura1) true false))))))

(event EventInteract
  (if (Variables|Default|Getroto)
    (CallFunction|Arreglar)))

(fn ConstructionScript)