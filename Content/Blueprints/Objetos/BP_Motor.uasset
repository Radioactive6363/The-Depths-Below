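; BP_Motor is an interactable engine that randomly breaks down and is repaired with an attached welding torch.
; While the torch is down, delayed Tick checks give a coin-flip chance to show three breaks if BP_ConsolaPoder is powered.
; Interacting when broken timeline-lerps the torch to the player, unless BP_TanqueOxigeno's tape is held.
; Further interactions hide breaks by name; clearing all three fixes the engine and returns the torch.
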(event Custom|Use
  ;[1 1 1] Accion Agarrar Soplete
  (if (Variables|Default|Getroto)
    (|ChequeoCintaenMano
      (:else
        (|AgarrarSoplete)))))

(event Custom|Soldar
  ;[1 1 1] Accion Arreglo
  (|ArregloRoturasIndividuales
    (:then
      _)
    (:then2
      _)
    (:then3
      _))
  (if (|CondicionArregloTotal)
    (Variables|Default|Setroto false)
    (|DevolverSoplete)))

(event EventBeginPlay
  (Variables|Default|Setroto false))

(event Collision|EventActorBeginOverlap
  (params (OtherActor :type Actor%20Object%20Reference)))

(event EventTick
  (params (DeltaSeconds :type Float%20%28single-precision%29))
  ;[1 1 1] Evento Random Rotura
  (if (not (Variables|Default|GetSopleteAgarrado))
    (Utilities|FlowControl|Delay 3e+01)
    (|ChequeoEncendido
      (:else
        (|50%ChanceRotura)))))

(event EventInteract
  ;[1 1 1] Interaccion inicial
  (if (Variables|Default|GetSopleteAgarrado)
    (CallFunction|Soldar)
    (else
      (CallFunction|Use))))

(fn ConstructionScript)