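; Breakable glass actor that runs the extraction phase and decides whether the run ends in victory or defeat.
; Once extraction starts, a 60-second window leads to victory, while a repeating delayed check re-shows six cracks if all were repaired, or triggers defeat.
; Interacting hides the crack matching NombreRotura.
; Both endings save a depth-based high score, 20% higher on victory, pause behind a result widget and pass scores to the game instance.
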(event Custom|Use
  ;[1 1 1] Arreglos
  (|ArregloRoturasIndividuales
    (:then
      _)
    (:then2
      _)
    (:then3
      _)
    (:then4
      _)
    (:then5
      _)
    (:then6
      _))
  (if (|CondicionArregloTotal)
    (Variables|Default|Setarreglo true)))

(event Custom|Rotura
  ;[1 1 1] Roturas
  (Utilities|FlowControl|Delay 5.0)
  (if (Variables|Default|Getarreglo)
    (|Roturas)
    (Variables|Default|Setarreglo false)
    (else
      (CallFunction|Derrota))))

(event Custom|Derrota
  ;[1 1 1] Pantalla Derrota
  (|GuardarPuntajeMaximo_2
    (:then
      _)
    (:then2
      _))
  (|PantallaDerrota)
  (|MostrarPuntaje_2))

(event Custom|Retirada
  ;[1 1 1] Ventana de Extraccion
  (Utilities|FlowControl|Delay 6e+01)
  (CallFunction|Victoria))

(event Custom|Victoria
  ;[1 1 1] Pantalla Victoria
  (|GuardarPuntajeMaximo
    (:then
      _)
    (:then2
      _))
  (|PantallaVictoria)
  (|MostrarPuntaje))

(event EventBeginPlay)

(event Collision|EventActorBeginOverlap
  (params (OtherActor :type Actor%20Object%20Reference)))

(event EventTick
  (params (DeltaSeconds :type Float%20%28single-precision%29))
  ;[1 1 1] Evento Chequeo Retirada
  (|ChequeoExtraccion)
  (|ObtenerProfMaxima)
  (CallFunction|Retirada))

(event EventInteract
  ;[1 1 1] Interaccion
  (CallFunction|Use))

(fn ConstructionScript)