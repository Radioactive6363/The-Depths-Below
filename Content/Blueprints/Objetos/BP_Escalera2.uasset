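; Interactable ladder that toggles the player on and off climbing on each Interact, setting the Escalera flag on BP_Personaje.
; A FlipFlop picks one of two collapsed graphs, with input disabled for a one-second delay before the flag changes.
; Mounting uses timelines to lerp the character to an offset from the ladder and turn the view toward it.
; Dismounting only turns the view toward an offset point and levels pitch.
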(event Custom|Use
  (bind _returnvalue (Game|GetPlayerController 0))
  (bind _returnvalue_2 (Game|GetPlayerCharacter 0))
  (bind _returnvalue_3 (Game|GetPlayerController 0))
  (bind _returnvalue_4 (Game|GetPlayerCharacter 0))
  (Utilities|FlowControl|FlipFlop
    (:A
      (Input|DisableInput _returnvalue_2 _returnvalue_3)
      (|MovimientoaEscalera)
      (Utilities|FlowControl|Delay 1.0)
      (Input|EnableInput _returnvalue_2 _returnvalue_3)
      (bind _asbp_personaje (Utilities|Casting|CastToBP_Personaje _returnvalue_2))
      (Variables|/Game/Blueprints/Personaje/BP_Personaje.BP_Personaje_C|SetEscalera _asbp_personaje true))
    (:B
      (Input|DisableInput _returnvalue_4 _returnvalue)
      (|MovimientodesdeEscalera)
      (Utilities|FlowControl|Delay 1.0)
      (Input|EnableInput _returnvalue_4 _returnvalue)
      (bind _asbp_personaje_2 (Utilities|Casting|CastToBP_Personaje _returnvalue_4))
      (Variables|/Game/Blueprints/Personaje/BP_Personaje.BP_Personaje_C|SetEscalera _asbp_personaje_2 false))))

(event EventBeginPlay)

(event Collision|EventActorBeginOverlap
  (params (OtherActor :type Actor%20Object%20Reference)))

(event EventTick
  (params (DeltaSeconds :type Float%20%28single-precision%29)))

(event EventInteract
  (CallFunction|Use))

(fn ConstructionScript)