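; Power console with a lever that the player interacts with to turn energy on, starting in the off state.
; Interaction is gated by BP_Motor's broken state, while Tick triggers shutdown based on the motor's repair flag and Extraccion.
; Timeline-based macros are meant to rotate the lever, swap indicator light materials and toggle point accrual on resource console widgets.
; Shutdown logic also stops the navigation actor's audio.
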(event Custom|Use
  ;[1 1 1] Accion de Encendido
  (|EncenderEnergia))

(event EventBeginPlay
  ;[1 1 1] Estado Inicial
  (Variables|Default|SetApagado true))

(event Collision|EventActorBeginOverlap
  (params (OtherActor :type Actor%20Object%20Reference)))

(event EventTick
  (params (DeltaSeconds :type Float%20%28single-precision%29))
  ;[1 1 1] Evento Apagado Energia
  (if (not (Variables|Default|Getextraccion))
    (if (not (Variables|Default|GetApagado))
      (|ChequeoMotor)
      (|ApagarEnergia))))

(event EventInteract
  ;[1 1 1] Interaccion
  (if (Variables|Default|GetApagado)
    (|ChequeoMotorRoto
      (:else
        (if (Variables|Default|Getinteracc)
          (CallFunction|Use)
          (Variables|Default|Setinteracc false))))))

(fn ConstructionScript)