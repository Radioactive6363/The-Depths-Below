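; Oxygen tank actor that drains over time, faster while broken, updates the resource console's status text at thresholds, and triggers defeat when empty.
; Interacting picks up tape (Cinta) via timelines, then patches named leaks; a three-second timer re-shows leaks during repair.
; Full repair stops leak audio, returns the tape and resets the sonar UI's active flag.
; Defeat saves max depth and best score, then pauses behind the defeat widget.
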(event Custom|Use
  ;[1 1 1] Accion Agarrar Cinta
  (if (Variables|Default|Getroto)
    (|ChequeoSopleteenMano
      (:else
        (|AgarrarCinta)))))

(event Custom|Rotura
  ;[1 1 1] Rotura
  (if (Variables|Default|GetCintaAgarrada)
    (if (|CondicionArranqueTimer)
      (|Ventanade3segundosparaarreglo))
    (elif (Variables|Default|Getinicial)
      (|RoturaInicial))))

(event Custom|Arreglar
  ;[1 1 1] Accion Arreglo
  (|ArregloRoturasIndividuales
    (:then
      _)
    (:then2
      _)
    (:then3
      _))
  (if (|CondicionArregloTotal)
    (Variables|Default|Setroto false)
    (Audio|Components|Audio|Stop (Variables|Default|GetGas%20Leak%20Audio))
    (|DevolverCinta)
    (Variables|Default|Setinicial true)
    (|ReactivarMonstruo)))

(event Custom|Muerte
  ;[1 1 1] Derrota
  (|ObtenerProfMaxima)
  (|GuardarPuntajeMaximo
    (:then
      _)
    (:then2
      _))
  (|PantallaDerrota)
  (|MostrarPuntaje))

(event EventBeginPlay)

(event Collision|EventActorBeginOverlap
  (params (OtherActor :type Actor%20Object%20Reference)))

(event EventTick
  (params (DeltaSeconds :type Float%20%28single-precision%29))
  (bind _oxigeno (Variables|Default|Getoxigeno))
  ;[1 1 1] Evento Random Rotura y Perdida de Oxigeno
  (if (> _oxigeno 0.0)
    (if (Variables|Default|Getroto)
      (CallFunction|Rotura)
      (|PerdidaOxigeno :!label _label)
      (else
        (goto _label execute2)))
    (elif (== _oxigeno 0.0)
      (CallFunction|Muerte))))

(event EventInteract
  ;[1 1 1] Interaccion Inicial
  (if (Variables|Default|GetCintaAgarrada)
    (CallFunction|Arreglar)
    (else
      (CallFunction|Use))))

(fn ConstructionScript)