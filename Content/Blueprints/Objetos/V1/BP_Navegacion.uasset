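; Interactable navigation station that lets the player set the vessel's speed with a lever (Cube5).
; Interact flip-flops between blending to the station's camera and returning to the character, restoring walking and pushing Velocidad to every BP_ConsolaRecursos widget.
; While active, Tick polls W/S to tilt the lever through timelines, locking input between steps.
; Lever pitch selects one of three Velocidad levels, stopping or swapping the underwater motor sound.
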(event Custom|Use
  ;[1 1 1] Accion Entrar y Salir
  (Utilities|FlowControl|FlipFlop
    (:A
      (|DeshabilitarInput)
      (|CambiarCamaraaNavegacionyHabilitarEjecucion)
      (|HabilitarInput))
    (:B
      (|DeshabilitarEjecucionyCambiarCamaraaPersonaje)
      (|SalirdeNavegacion))))

(event Custom|setVelocidad
  (bind (_returnvalue _returnvalue2) (|DireccionMovimiento))
  ;[1 1 1] Cambiar Velocidad
  (if (not (Variables|Default|Getdelay))
    (if _returnvalue
      (if (|RotacionMaxima)
        (bind _returnvalue_2 (|SubirPalanca))
        (|VelocidadEstablecida (.ReturnValue (|VelocidadSeleccionada _returnvalue_2 _returnvalue_2 _returnvalue_2 _returnvalue_2)) (.ReturnValue2 (|VelocidadSeleccionada _returnvalue_2 _returnvalue_2 _returnvalue_2 _returnvalue_2)) (.ReturnValue3 (|VelocidadSeleccionada _returnvalue_2 _returnvalue_2 _returnvalue_2 _returnvalue_2)) :!label _label))
      (elif _returnvalue2
        (if (|RotacionMinima)
          (|BajarPalanca)
          (goto _label))))))

(event EventBeginPlay)

(event Collision|EventActorBeginOverlap
  (params (OtherActor :type Actor%20Object%20Reference)))

(event EventTick
  (params (DeltaSeconds :type Float%20%28single-precision%29))
  ;[1 1 1] Ejecucion Cambio de Velocidad
  (if (Variables|Default|GetInteracc)
    (CallFunction|SetVelocidad)))

(event EventInteract
  ;[1 1 1] Interaccion
  (CallFunction|Use))

(fn ConstructionScript)