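; BP_ConsolaRecursos is an interactable resource console with a widget UI and text input.
; Each interaction toggles via FlipFlop between a blended console camera with Game-and-UI input and keyboard focus, and the player view with game-only input.
; Both states hide the cursor and set BP_Personaje's Mouse flag false.
; On BeginPlay it loads the maximum depth record from BP_Vidrio's save slot into the widget.
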(event Custom|Use
  ;[1 1 1] Accion Entrar y Salir
  (Utilities|FlowControl|FlipFlop
    (:A
      (|CambiarCamaraaConsola)
      (|ModoInputUI)
      (|EstablecerEstadoMouseActivoenPersonaje))
    (:B
      (|CambiarCamaraaPersonaje)
      (|ModoInputJuego)
      (|EstablecerEstadoMouseInactivoenPersonaje))))

(event EventBeginPlay
  (|CargarPuntajeMaximo))

(event Collision|EventActorBeginOverlap
  (params (OtherActor :type Actor%20Object%20Reference)))

(event EventTick
  (params (DeltaSeconds :type Float%20%28single-precision%29)))

(event EventInteract
  ;[1 1 1] Interaccion
  (CallFunction|Use))

(fn ConstructionScript)