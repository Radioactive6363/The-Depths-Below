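; Interactable ladder that puts the player into and out of ladder state, alternating on each Interact through a FlipFlop.
; Entry uses timelines to slide the player to a fixed world-X offset and turn the view toward the ladder, then sets BP_Personaje's Escalera flag.
; Exit turns the view, clears Escalera and EstadoInteract, and restores Walking.
; Both transitions disable player input and re-enable it after a short delay.
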(event Custom|Use
  ;[1 1 1] Accion Ingreso y Egreso
  (Utilities|FlowControl|FlipFlop
    (:A
      (bind (_returnvalue _returnvalue2) (|DeshabilitarInputHaciaEscalera))
      (|MovimientoaEscalera)
      (|DelaydeInputDuranteIngresoaEscalera _returnvalue _returnvalue2)
      (|HabilitarEstadoEscaleraenPersonaje _returnvalue))
    (:B
      (bind (_returnvalue_2 _returnvalue2_2) (|DeshabilitarInputDesdeEscalera))
      (|MovimientodesdeEscalera)
      (|DelaydeInputDuranteEgresodesdeEscalera _returnvalue_2 _returnvalue2_2)
      (|DeshabilitarEstadoEscaleraenPersonaje _returnvalue_2))))

(event EventBeginPlay)

(event Collision|EventActorBeginOverlap
  (params (OtherActor :type Actor%20Object%20Reference)))

(event EventTick
  (params (DeltaSeconds :type Float%20%28single-precision%29)))

(event EventInteract
  ;[1 1 1] Interaccion
  (CallFunction|Use))

(fn ConstructionScript)