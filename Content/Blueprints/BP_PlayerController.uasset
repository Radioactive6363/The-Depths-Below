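; Player controller that sets up the player HUD and handles input for toggling on-screen widgets.
; On BeginPlay it adds the widget Enhanced Input mapping context, creates the HUD and binds its in-game controls widget to event dispatchers.
; Input actions fire those dispatchers to show or hide controls and hide option buttons, decoupling input from UI.
; A further input action runs the Stat FPS console command.
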(event Custom|BindEventsUI
  (Utilities|IsValid (Variables|/Game/Blueprints/UI/BP_PlayerHUD.BP_PlayerHUD_C|GetBP_ControlsInGame (Variables|Default|GetPlayerHUD))
    (:Is%20Valid
      (EventDispatchers|BindEventtoShow/HideControls (EventDispatchers|CreateEvent (Variables|/Game/Blueprints/UI/BP_PlayerHUD.BP_PlayerHUD_C|GetBP_ControlsInGame (Variables|Default|GetPlayerHUD)) :!event Show/HideControlsUI))
      (EventDispatchers|BindEventtoHideButtonOptions (EventDispatchers|CreateEvent (Variables|/Game/Blueprints/UI/BP_PlayerHUD.BP_PlayerHUD_C|GetBP_ControlsInGame (Variables|Default|GetPlayerHUD)) :!event HideControlsText)))))

(event Input|EnhancedActionEvents|EnhancedInputActionIA_ShowControls
  (params (ActionValue :type Boolean) (ElapsedSeconds :type Float%20%28double-precision%29) (TriggeredSeconds :type Float%20%28double-precision%29) (InputAction :type Input%20Action%20Object%20Reference :default "/Game/Inputs/IA_ShowControls.IA_ShowControls"))
  (Default|CallShow/HideControls))

(event Input|EnhancedActionEvents|EnhancedInputActionIA_HideButtonOptions
  (params (ActionValue :type Boolean) (ElapsedSeconds :type Float%20%28double-precision%29) (TriggeredSeconds :type Float%20%28double-precision%29) (InputAction :type Input%20Action%20Object%20Reference :default "/Game/Inputs/IA_HideButtonOptions.IA_HideButtonOptions"))
  (Default|CallHideButtonOptions))

(event Input|EnhancedActionEvents|EnhancedInputActionIA_ActivateFPS
  (params (ActionValue :type Boolean) (ElapsedSeconds :type Float%20%28double-precision%29) (TriggeredSeconds :type Float%20%28double-precision%29) (InputAction :type Input%20Action%20Object%20Reference :default "/Game/Inputs/IA_ActivateFPS.IA_ActivateFPS"))
  (Development|ExecuteConsoleCommand "Stat FPS" (Game|GetPlayerController 0)))

(event EventBeginPlay
  (Utilities|FlowControl|Sequence
    (:then_0
      (Input|AddMappingContext (PlayerController|LocalPlayerSubsystems|GetEnhancedInputLocalPlayerSubsystem) "/Game/Inputs/IMC_PlayerWidgets.IMC_PlayerWidgets" 0 "(bIgnoreAllPressedKeysUntilRelease=True,bForceImmediately=False,bNotifyUserSettings=False)"))
    (:then_1
      (bind _returnvalue (Game|ConstructObjectfromClass "/Game/Blueprints/UI/BP_PlayerHUD.BP_PlayerHUD_C"))
      (bind _output_get (Variables|Default|SetPlayerHUD _returnvalue))
      (UserInterface|Viewport|AddtoViewport _output_get 0)
      (CallFunction|BindEventsUI))))

(fn ConstructionScript)